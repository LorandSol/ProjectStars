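; HG_GameInstance is a game instance Blueprint that persists the player's master volume setting in an options save game.
; The LoadOptions macro loads the SV_Options object from its save slot, or creates a new one when no save exists, and caches it in SVOptions.
; SaveAudioSettings runs that macro, writes the new MasterVolume into the cached object and saves it back to the same slot.
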(event `/Game/Blueprints/PlayerCharacter/BPI_GameInstance.SaveAudioSettings`
  (params (`Master Volume` :type "Float (double-precision)"))
  (`self.LoadOptions`
    (:`OutputPin`
      (set `/Game/Blueprints/PlayerCharacter/SaveFiles/SV_Options.Master Volume` `Master Volume` (`self.SV Options`))
      (`GameplayStatics.SaveGameToSlot` (`self.SV Options`) (`self.Options Save Slot`)))))