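; Interactable hiding spot that lets L1_Character hide under an object and blends the view to this actor.
; A box overlap enables input and opens a gate, so HideUnder toggles between the character's HideUnder and UnHideUnder.
; While hiding, look input accumulates into clamped pitch and yaw instead of driving the controller.
; MoveCamera is empty and the rotation loop that would apply those angles is disconnected.
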(event `InputAction|HideUnder`
  (params (Key :type "Key Structure"))
  (bind _character_ref (`self.Character Ref`))
  (:`Pressed`
    (`/Engine/EditorBlueprintResources/StandardMacros.Gate` true :!label _label
      (:`Exit`
        (if (`/Game/Blueprints/PlayerCharacter/Level1/L1_Character.isHiding` _character_ref)
          (`/Game/Blueprints/PlayerCharacter/Level1/L1_Character.UnHideUnder` _character_ref)
          (else
            (`/Game/Blueprints/PlayerCharacter/Level1/L1_Character.HideUnder` _character_ref)
            (`|ExecutionSequence`
              (:`then_0`
                (`PlayerController.SetViewTargetWithBlend` (`GameplayStatics.GetPlayerController` 0) self 0.5 "VTBlend_Linear" 0.0 false)
                (`self.MoveCamera`))
              (:`then_1`
                (`KismetSystemLibrary.Delay` 0.2)
                (`self.EnableInput` (`GameplayStatics.GetPlayerController` 0) :!label _label_2)
                (goto _label :!via `Open`)))))))))

(event `self.Box.OnComponentBeginOverlap`
  (params (OverlappedComponent :type "PrimitiveComponent Object Reference") (OtherActor :type "Actor Object Reference") (OtherComp :type "PrimitiveComponent Object Reference") (OtherBodyIndex :type Integer) (bFromSweep :type Boolean) (SweepResult :type "HitResult Structure (by ref)"))
  (bind _asl1_character (cast `/Game/Blueprints/PlayerCharacter/Level1/L1_Character` OtherActor))
  (set `self.Character Ref` _asl1_character)
  (goto _label_2))

(event `self.Box.OnComponentEndOverlap`
  (params (OverlappedComponent :type "PrimitiveComponent Object Reference") (OtherActor :type "Actor Object Reference") (OtherComp :type "PrimitiveComponent Object Reference") (OtherBodyIndex :type Integer))
  (cast `/Game/Blueprints/PlayerCharacter/Level1/L1_Character` OtherActor)
  (`self.DisableInput` (`GameplayStatics.GetPlayerController` 0))
  (goto _label :!via `Close`))

(event `MovePlayer`)

(event `MoveCamera`)

(event `InputAxis|LookUp`
  (params (AxisValue :type "Float (single-precision)"))
  (bind _character_ref (`self.Character Ref`))
  (if (`/Game/Blueprints/PlayerCharacter/Level1/L1_Character.isHiding` _character_ref)
    (bind _output_get (set `self.Pitch` (+ (`self.Pitch`) AxisValue)))
    (bind _output_get_2 (set `self.Pitch` (`KismetMathLibrary.FClamp` _output_get -10.0 10.0)))
    (else
      (`Pawn.AddControllerPitchInput` _character_ref AxisValue))))

(event `InputAxis|Turn`
  (params (AxisValue :type "Float (single-precision)"))
  (bind _character_ref (`self.Character Ref`))
  (if (`/Game/Blueprints/PlayerCharacter/Level1/L1_Character.isHiding` _character_ref)
    (bind _output_get (set `self.Yaw` (+ (`self.Yaw`) AxisValue)))
    (bind _output_get_2 (set `self.Yaw` (`KismetMathLibrary.FClamp` _output_get 260.0 300.0)))
    (else
      (`Pawn.AddControllerYawInput` _character_ref AxisValue))))

(fn `UserConstructionScript`)