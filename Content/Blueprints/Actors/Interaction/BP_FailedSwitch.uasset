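; Interactable switch, apparently a picture frame, that on Interact slides a referenced BookShelf mesh, tilts itself, then resets as a failed attempt.
; A timeline adds a lerped offset to the shelf's current world location each update along X or Y, so movement accumulates.
; It also drives the tilt timeline, followed once by a delay, bell sound at world origin and tilt-back.
; IsOpen blocks repeat interaction and is never cleared.
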(event `self.ReceiveBeginPlay`
  (`parent.ReceiveBeginPlay`))

(event `self.Interact`
  (bind _staticmeshcomponent (`StaticMeshActor.StaticMeshComponent` (`self.BookShelf`)))
  (bind (_returnvalue_x _returnvalue_y _returnvalue_z) (`KismetMathLibrary.BreakVector` (`SceneComponent.K2_GetComponentLocation` _staticmeshcomponent)))
  (bind (_returnvalue_x_2 _returnvalue_y_2 _returnvalue_z_2) (`KismetMathLibrary.BreakVector` (`SceneComponent.K2_GetComponentLocation` _staticmeshcomponent)))
  ;[1 1 1] Moves static mesh (make sure static mesh is set to movable)
  (`/Engine/EditorBlueprintResources/StandardMacros.IsValid` (`self.BookShelf`) ; makes sure the reference is valid
    (:`Is Valid`
      (if (not (`self.isOpen`))
        (bind (_direction _alpha) (`Timeline|Timeline`) ; creates a small animation so the object doesn't snap to position
          (:`Update`
            (if (`self.Yaxis`)
              (bind _returnvalue (`KismetMathLibrary.Lerp` 0.0 (`self.MoveObject`) _alpha))
              (`SceneComponent.K2_SetRelativeLocation` _staticmeshcomponent (`KismetMathLibrary.MakeVector` _returnvalue_x (+ _returnvalue_y _returnvalue) _returnvalue_z) false false)
              (else
                (`SceneComponent.K2_SetRelativeLocation` _staticmeshcomponent (`KismetMathLibrary.MakeVector` (+ _returnvalue_x_2 _returnvalue) _returnvalue_y_2 _returnvalue_z_2) false false)))
            (set `self.isOpen` true)
            (bind (_direction_2 _alpha_2) (`Timeline|PictureFrame`)
              (:`Update`
                (`SceneComponent.K2_SetRelativeRotation` (`self.StaticMesh`) (`KismetMathLibrary.MakeRotator` 90.0 (`KismetMathLibrary.Lerp` 0.0 20.0 _alpha_2)) false false)
                (`/Engine/EditorBlueprintResources/StandardMacros.DoOnce` false
                  (:`Completed`
                    (`KismetSystemLibrary.Delay` 1.0)
                    (`GameplayStatics.PlaySoundAtLocation` "/Game/Sounds/Misc/Bell.Bell" (0.0 0.0 0.0) (struct) 1.0 1.0 0.0 null null null null)
                    (bind (_direction_3 _alpha_3) (`Timeline|Fail`)
                      (:`Update`
                        (`SceneComponent.K2_SetRelativeRotation` (`self.StaticMesh`) (`KismetMathLibrary.MakeRotator` 90.0 (`KismetMathLibrary.Lerp` 20.0 0.0 _alpha_3)) false false)))))))))))))

(fn `UserConstructionScript`
  (`parent.UserConstructionScript`))