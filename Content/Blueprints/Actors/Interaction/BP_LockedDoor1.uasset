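; Locked exit door that ends the game with a survival screen when an L1_Character enters its box holding the key.
; Overlap requires both the player's HasKey and the door's own HasKey, set by PickUpkey, otherwise it plays a locked sound.
; On success it clears the player's objective, pauses, removes all widgets including the just-added OpenDoor widget, then shows YouSurvivedWidget and the mouse cursor.
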(event `self.Box.OnComponentBeginOverlap`
  (params (OverlappedComponent :type "PrimitiveComponent Object Reference") (OtherActor :type "Actor Object Reference") (OtherComp :type "PrimitiveComponent Object Reference") (OtherBodyIndex :type Integer) (bFromSweep :type Boolean) (SweepResult :type "HitResult Structure (by ref)"))
  (bind _returnvalue (`GameplayStatics.GetPlayerController` 0))
  (bind _playerref (`self.PlayerRef`))
  (bind _asl1_character (cast `/Game/Blueprints/PlayerCharacter/Level1/L1_Character` OtherActor))
  (bind _output_get (set `self.PlayerRef` _asl1_character))
  (`/Engine/EditorBlueprintResources/StandardMacros.IsValid` _playerref
    (:`Is Valid`
      _)
    (:`Is Not Valid`
      (set `self.PlayerRef` _output_get)))
  (if (and (`/Game/Blueprints/PlayerCharacter/Level1/L1_Character.HasKey` _playerref) (`self.HasKey?`))
    (if true
      (bind _returnvalue_2 (`|CreateWidget` "/Game/Widgets/OpenDoor_Widget.OpenDoor_Widget_C"))
      (bind _output_get_2 (set `self.Open door` _returnvalue_2))
      (`UserWidget.AddToViewport` _output_get_2 0)
      (set `/Game/Blueprints/PlayerCharacter/Level1/L1_Character.PlayerHasAnObjective` false (`self.PlayerRef`))
      (`GameplayStatics.SetGamePaused` true)
      (`WidgetLayoutLibrary.RemoveAllWidgets`)
      (bind _returnvalue_3 (`|CreateWidget` "/Game/Widgets/YouSurvivedWidget.YouSurvivedWidget_C" _returnvalue))
      (`UserWidget.AddToViewport` _returnvalue_3 0)
      (set `PlayerController.bShowMouseCursor` true _returnvalue))
    (else
      (`GameplayStatics.PlaySound2D` "/Game/Sounds/Mechanics/doorLocked.doorLocked" 1.0 1.0 0.0 null null))))

(event `/Game/Blueprints/Interface/BPI_Door.PickUpkey`
  (set `self.HasKey?` true))

(fn `UserConstructionScript`)