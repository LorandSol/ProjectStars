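; Interactable locked double door that requires the player to have a key and an active objective to unlock.
; Without the key, Interact plays a locked sound and shows a prompt widget, removed on leaving the trigger box.
; Once unlocked, later interactions pass an overlap-controlled Gate into a FlipFlop, alternately swinging both leaves open and closed via timelines and a delayed Open flag.
; Older direction-aware swing logic remains unconnected.
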(event `/Game/Blueprints/Interface/BPI_Interaction.Interact`
  (if (not (`self.PlayerOpenedDoor`))
    (bind _asl1_character (cast `/Game/Blueprints/PlayerCharacter/Level1/L1_Character` (`GameplayStatics.GetPlayerCharacter` 0)))
    (bind _output_get (set `self.PlayerRef` _asl1_character))
    (`/Engine/EditorBlueprintResources/StandardMacros.IsValid` _output_get
      (:`Is Valid`
        _)
      (:`Is Not Valid`
        (bind _output_get_2 (set `self.PlayerRef` _output_get))))
    (if (`/Game/Blueprints/PlayerCharacter/Level1/L1_Character.HasKey` _output_get_2)
      (if (`/Game/Blueprints/PlayerCharacter/Level1/L1_Character.PlayerHasAnObjective` _output_get)
        (set `self.PlayerOpenedDoor` true)
        (set `/Game/Blueprints/PlayerCharacter/Level1/L1_Character.PlayerHasAnObjective` false (`self.PlayerRef`)))
      (else
        (`GameplayStatics.PlaySound2D` "/Game/Sounds/Mechanics/doorLocked.doorLocked" 1.0 1.0 0.0 null null)
        (if (not (`self.DoorWidgetPrinted`))
          (set `self.Tried to open door` true)
          (bind _returnvalue (`|CreateWidget` "/Game/Widgets/OpenDoor_Widget.OpenDoor_Widget_C"))
          (bind _output_get_3 (set `self.OpenDoorWidget` _returnvalue))
          (`UserWidget.AddToViewport` _output_get_3 0)
          (set `self.DoorWidgetPrinted` true))))
    (else
      (`/Engine/EditorBlueprintResources/StandardMacros.Gate` true :!label _label
        (:`Exit`
          (`/Engine/EditorBlueprintResources/StandardMacros.FlipFlop`
            (:`A`
              (if (not (`self.Open?`))
                ;[1 1 1] Door Open
                (`|ExecutionSequence`
                  (:`then_0`
                    (bind (_direction _leftdooropen) (`Timeline|Left Door Open` :!via `PlayFromStart`)
                      (:`Update`
                        (`SceneComponent.K2_SetRelativeRotation` (`self.Door2`) (`KismetMathLibrary.MakeRotator` 0.0 0.0 (`KismetMathLibrary.Lerp` (`self.LeftDoorClosedFloat`) (`self.LeftDoorOpenFloat`) _leftdooropen)) false false))))
                  (:`then_1`
                    (bind (_direction_2 _rightdooropen) (`Timeline|RightDoorOpen` :!via `PlayFromStart`)
                      (:`Update`
                        (`SceneComponent.K2_SetRelativeRotation` (`self.Door1`) (`KismetMathLibrary.MakeRotator` 0.0 0.0 (`KismetMathLibrary.Lerp` (`self.RightDoorClosedFloat`) (`self.RightDoorOpenFloat`) _rightdooropen)) false false)))))
                (`KismetSystemLibrary.Delay` 3.0)
                (set `self.Open?` true)))
            (:`B`
              (if (`self.Open?`)
                ;[1 1 1] Door Close
                (`|ExecutionSequence`
                  (:`then_0`
                    (bind (_direction_3 _leftdooropen_2) (`Timeline|Timeline_1` :!via `ReverseFromEnd`)
                      (:`Update`
                        (`SceneComponent.K2_SetRelativeRotation` (`self.Door2`) (`KismetMathLibrary.MakeRotator` 0.0 0.0 (`KismetMathLibrary.Lerp` (`self.LeftDoorClosedFloat`) (`self.LeftDoorOpenFloat`) _leftdooropen_2)) false false))))
                  (:`then_1`
                    (bind (_direction_4 _rightdooropen_2) (`Timeline|Timeline_2` :!via `ReverseFromEnd`)
                      (:`Update`
                        (`SceneComponent.K2_SetRelativeRotation` (`self.Door1`) (`KismetMathLibrary.MakeRotator` 0.0 0.0 (`KismetMathLibrary.Lerp` (`self.RightDoorClosedFloat`) (`self.RightDoorOpenFloat`) _rightdooropen_2)) false false)))))
                (`KismetSystemLibrary.Delay` 3.0)
                (set `self.Open?` false)))))))))

(event `/Game/Blueprints/Interface/BPI_Door.PickUpkey`
  (set `self.HasKey?` true))

(event `self.Box.OnComponentBeginOverlap`
  (params (OverlappedComponent :type "PrimitiveComponent Object Reference") (OtherActor :type "Actor Object Reference") (OtherComp :type "PrimitiveComponent Object Reference") (OtherBodyIndex :type Integer) (bFromSweep :type Boolean) (SweepResult :type "HitResult Structure (by ref)"))
  (`SceneComponent.SetVisibility` (`self.Widget`) true false)
  (cast `/Game/Blueprints/PlayerCharacter/Level1/L1_Character` OtherActor)
  (goto _label :!via `Open`))

(event `self.Box.OnComponentEndOverlap`
  (params (OverlappedComponent :type "PrimitiveComponent Object Reference") (OtherActor :type "Actor Object Reference") (OtherComp :type "PrimitiveComponent Object Reference") (OtherBodyIndex :type Integer))
  (`SceneComponent.SetVisibility` (`self.Widget`) false false)
  (if (`self.Tried to open door`)
    (`Widget.RemoveFromParent` (`self.OpenDoorWidget`))
    (set `self.Tried to open door` false)
    (set `self.DoorWidgetPrinted` false)
    (cast `/Game/Blueprints/PlayerCharacter/Level1/L1_Character` OtherActor)
    (goto _label :!via `Close`)))

(fn `UserConstructionScript`
  (`parent.UserConstructionScript`))