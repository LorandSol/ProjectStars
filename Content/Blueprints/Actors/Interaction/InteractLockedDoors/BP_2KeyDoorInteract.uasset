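; Locked interactable door that opens only when the player's L1_Character holds at least KeysRequired key parts.
; Interact toggles it with sound, playing or reversing a Timeline that lerps the door's yaw.
; A dot product on opening picks the swing direction from the player's side.
; Without enough keys, it plays a locked sound and shows a single need-more-keys widget, removed when the Box overlap ends.
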(event `/Game/Blueprints/Interface/BPI_Interaction.Interact`
  (bind _returnvalue (`self.K2_GetActorLocation`))
  (bind _asl1_character (cast `/Game/Blueprints/PlayerCharacter/Level1/L1_Character` (`GameplayStatics.GetPlayerCharacter` 0)))
  (if (>= (`/Game/Blueprints/PlayerCharacter/Level1/L1_Character.KeyPart_TotalAmount` _asl1_character) (`self.KeysRequired`))
    (if (`self.IsDoorClosed`)
      (set `self.IsDoorClosed` false)
      (`GameplayStatics.PlaySoundAtLocation` "/Game/Sounds/Misc/CloseDoor.CloseDoor" _returnvalue (struct) 1.0 1.0 0.0 null null null null)
      (bind (_direction _alpha) (`Timeline|Timeline` :!via `Reverse` :!label _label)
        (:`Update`
          (`SceneComponent.K2_SetRelativeRotation` (`self.Door`) (`KismetMathLibrary.MakeRotator` 0.0 0.0 (`KismetMathLibrary.Lerp` 0.0 (select `bool` (>= (`self.DotProduct`) 0.0) :`false` -85.0 :`true` 85.0) _alpha)) false false)))
      (else
        (set `self.IsDoorClosed` true)
        (`GameplayStatics.PlaySoundAtLocation` "/Game/Sounds/Misc/OpenDoor.OpenDoor" _returnvalue (struct) 1.0 1.0 0.0 null null null null)
        (set `self.DotProduct` (`KismetMathLibrary.Dot_VectorVector` (`KismetMathLibrary.Normal` (- (`self.K2_GetActorLocation` self) (`self.K2_GetActorLocation` _asl1_character))) (`self.GetActorForwardVector` self)))
        (goto _label)))
    (else
      (`GameplayStatics.PlaySoundAtLocation` "/Game/Sounds/Mechanics/WavFiles/doorLocked.doorLocked" _returnvalue (struct) 1.0 1.0 0.0 null null null null)
      (if (not (`self.NeedMoreKeysPrinted`))
        (bind _returnvalue_2 (`|CreateWidget` "/Game/Widgets/Need2MoreKeys_Widget.Need2MoreKeys_Widget_C"))
        (bind _output_get (set `self.NeedMoreKeys` _returnvalue_2))
        (`UserWidget.AddToViewport` _output_get 0)
        (set `self.NeedMoreKeysPrinted` true)))))

(event `self.Box.OnComponentBeginOverlap`
  (params (OverlappedComponent :type "PrimitiveComponent Object Reference") (OtherActor :type "Actor Object Reference") (OtherComp :type "PrimitiveComponent Object Reference") (OtherBodyIndex :type Integer) (bFromSweep :type Boolean) (SweepResult :type "HitResult Structure (by ref)")))

(event `self.Box.OnComponentEndOverlap`
  (params (OverlappedComponent :type "PrimitiveComponent Object Reference") (OtherActor :type "Actor Object Reference") (OtherComp :type "PrimitiveComponent Object Reference") (OtherBodyIndex :type Integer))
  (`Widget.RemoveFromParent` (stale `/Game/Blueprints/Interface/BPI_Interaction.Interact` _returnvalue_2))
  (set `self.NeedMoreKeysPrinted` false))

(fn `UserConstructionScript`)