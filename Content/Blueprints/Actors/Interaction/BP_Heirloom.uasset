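; BP_Heirloom is an interactable pickup actor that gives the player the heirloom and a new objective.
; A box overlap shows and hides its widget.
; On Interact, it flags HasHeirloom on the L1_Character and clears PlayerHasAnObjective, so the following check always passes.
; It then assigns its Objective as the current one, plays a 2D sound and destroys itself.
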(event `self.Box.OnComponentBeginOverlap`
  (params (OverlappedComponent :type "PrimitiveComponent Object Reference") (OtherActor :type "Actor Object Reference") (OtherComp :type "PrimitiveComponent Object Reference") (OtherBodyIndex :type Integer) (bFromSweep :type Boolean) (SweepResult :type "HitResult Structure (by ref)"))
  (`SceneComponent.SetVisibility` (`self.Widget`) true false))

(event `self.Box.OnComponentEndOverlap`
  (params (OverlappedComponent :type "PrimitiveComponent Object Reference") (OtherActor :type "Actor Object Reference") (OtherComp :type "PrimitiveComponent Object Reference") (OtherBodyIndex :type Integer))
  (`SceneComponent.SetVisibility` (`self.Widget`) false false))

(event `/Game/Blueprints/Interface/BPI_Interaction.Interact`
  (bind _asl1_character (cast `/Game/Blueprints/PlayerCharacter/Level1/L1_Character` (`GameplayStatics.GetPlayerCharacter` 0)))
  (bind _output_get (set `self.As L1 Character` _asl1_character))
  (set `/Game/Blueprints/PlayerCharacter/Level1/L1_Character.HasHeirloom` true _output_get)
  (set `/Game/Blueprints/PlayerCharacter/Level1/L1_Character.PlayerHasAnObjective` false _asl1_character)
  (if (not (`/Game/Blueprints/PlayerCharacter/Level1/L1_Character.PlayerHasAnObjective` _asl1_character))
    (set `/Game/Blueprints/PlayerCharacter/Level1/L1_Character.CurrentObjective` (`self.Objective`) _asl1_character)
    (set `/Game/Blueprints/PlayerCharacter/Level1/L1_Character.PlayerHasAnObjective` true _asl1_character)
    (`GameplayStatics.PlaySound2D` "/Game/Sounds/Mechanics/objective2.objective2" 1.0 1.0 0.0 null null)
    (`self.K2_DestroyActor`)))

(fn `UserConstructionScript`
  (`parent.UserConstructionScript`))