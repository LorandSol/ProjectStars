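; BP_LockedKeyDoor_OpenAway is a locked door that ends the game in survival once the player opens it with a key.
; Its Box overlap checks HasKey on L1_Character, showing a find-the-key widget without it, or playing a timeline that yaws the Door with it.
; The timeline's Update also runs a one-second Delay, then pauses, swaps in the YouSurvived widget and shows the cursor.
; Any end overlap removes all widgets.
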(event `self.Box.OnComponentBeginOverlap`
  (params (OverlappedComponent :type "PrimitiveComponent Object Reference") (OtherActor :type "Actor Object Reference") (OtherComp :type "PrimitiveComponent Object Reference") (OtherBodyIndex :type Integer) (bFromSweep :type Boolean) (SweepResult :type "HitResult Structure (by ref)"))
  (bind _returnvalue (`GameplayStatics.GetPlayerController` 0))
  (bind _asl1_character (cast `/Game/Blueprints/PlayerCharacter/Level1/L1_Character` OtherActor))
  (if (`/Game/Blueprints/PlayerCharacter/Level1/L1_Character.HasKey` _asl1_character)
    (bind (_direction _doorrotation) (`Timeline|DoorRotation`)
      (:`Update`
        (`SceneComponent.K2_SetRelativeRotation` (`self.Door`) (`KismetMathLibrary.MakeRotator` 0.0 0.0 _doorrotation) false false)
        (`KismetSystemLibrary.Delay` 1.0)
        (`GameplayStatics.SetGamePaused` true)
        (`WidgetLayoutLibrary.RemoveAllWidgets`)
        (bind _returnvalue_2 (`|CreateWidget` "/Game/Widgets/YouSurvivedWidget.YouSurvivedWidget_C" _returnvalue))
        (`UserWidget.AddToViewport` _returnvalue_2 0)
        (set `PlayerController.bShowMouseCursor` true _returnvalue)))
    (else
      (bind _returnvalue_3 (`|CreateWidget` "/Game/Widgets/FindTheKey_Widget.FindTheKey_Widget_C"))
      (`UserWidget.AddToViewport` _returnvalue_3 0))))

(event `self.Box.OnComponentEndOverlap`
  (params (OverlappedComponent :type "PrimitiveComponent Object Reference") (OtherActor :type "Actor Object Reference") (OtherComp :type "PrimitiveComponent Object Reference") (OtherBodyIndex :type Integer))
  (`WidgetLayoutLibrary.RemoveAllWidgets`))

(fn `UserConstructionScript`
  (`parent.UserConstructionScript`))