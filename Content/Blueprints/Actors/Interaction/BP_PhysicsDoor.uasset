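; BP_PhysicsDoor is a door actor apparently intended to be grabbed and swung with horizontal look input, but its logic is currently disconnected.
; GrabObject, ReleaseObject, MoveDoor and the LookRight axis event are all empty.
; Unwired nodes would lock player movement and look while enabling door input, restore them on release, and feed scaled axis input into Door yaw.
; That yaw flips sign by the player's side, using a dot product, without physics simulation.
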(event `/Game/Blueprints/Interface/BPI_Grab.GrabObject`)

(event `MoveDoor`
  (params (Amount :type "Float (double-precision)")))

(event `InputAxis|LookRight`
  (params (AxisValue :type "Float (single-precision)")))

(event `/Game/Blueprints/Interface/BPI_Grab.ReleaseObject`)

(fn `UserConstructionScript`)