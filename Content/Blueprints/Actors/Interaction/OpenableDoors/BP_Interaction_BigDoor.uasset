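; Locked double door that the player unlocks with a key as part of an objective.
; Interacting without the key shows a locked message and an objective pop-up, while having key and objective unlocks every BigDoor instance.
; Once unlocked, interaction toggles a timeline swinging both leaves away from the player, using a dot product for direction.
; A trigger box toggles the prompt widget; the monster door-opening logic is disconnected.
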(event `/Game/Blueprints/Interface/BPI_Interaction.Interact`
  (bind _returnvalue (`self.K2_GetActorLocation`))
  (if (not (`self.PlayerOpenedDoor`))
    (bind _asl1_character (cast `/Game/Blueprints/PlayerCharacter/Level1/L1_Character` (`GameplayStatics.GetPlayerCharacter` 0)))
    (bind _output_get (set `self.PlayerRef` _asl1_character))
    (`/Engine/EditorBlueprintResources/StandardMacros.IsValid` _output_get
      (:`Is Valid`
        _)
      (:`Is Not Valid`
        (bind _output_get_2 (set `self.PlayerRef` _output_get))))
    (if (`/Game/Blueprints/PlayerCharacter/Level1/L1_Character.HasKey` _output_get_2)
      (if (`/Game/Blueprints/PlayerCharacter/Level1/L1_Character.PlayerHasAnObjective` _output_get)
        (bind _outactors (`GameplayStatics.GetAllActorsOfClass` "BP_Interaction_BigDoor_C"))
        (bind _output_get_3 (set `self.BP_Doors` _outactors))
        (for _array_element _output_get_3
          (set `/Game/Blueprints/Actors/Interaction/OpenableDoors/BP_Interaction_BigDoor.PlayerOpenedDoor` true _array_element)
          (set `/Game/Blueprints/PlayerCharacter/Level1/L1_Character.PlayerHasAnObjective` false (`self.PlayerRef`))))
      (else
        (`GameplayStatics.PlaySound2D` "/Game/Sounds/Mechanics/WavFiles/doorLocked.doorLocked" 1.0 1.0 0.0 null null)
        (if (not (`self.DoorWidgetPrinted`))
          (set `self.Tried to open door` true)
          (bind _returnvalue_2 (`|CreateWidget` "/Game/Widgets/OpenDoor_Widget.OpenDoor_Widget_C"))
          (bind _output_get_4 (set `self.OpenDoorWidget` _returnvalue_2))
          (`UserWidget.AddToViewport` _output_get_4 0)
          (set `self.DoorWidgetPrinted` true)
          (`KismetSystemLibrary.Delay` 2.0)
          (if (not (`self.ObjectivePicked`))
            (`/Engine/EditorBlueprintResources/StandardMacros.DoOnce` false
              (:`Completed`
                (bind _returnvalue_3 (`|CreateWidget` "/Game/Widgets/Objectives/ObjectivePopUp.ObjectivePopUp_C"))
                (bind _output_get_5 (set `self.ObjectivePopUp` _returnvalue_3))
                (`UserWidget.AddToViewport` _output_get_5 0)
                (`GameplayStatics.PlaySound2D` "/Game/Sounds/Mechanics/WavFiles/scribble.scribble" 1.0 1.0 0.0 null null)
                (for _array_element_2 (`self.BP_Doors`)
                  (set `/Game/Blueprints/Actors/Interaction/OpenableDoors/BP_Interaction_BigDoor.ObjectivePicked` true _array_element_2))))))))
    (elif true
      (if (`self.IsDoorClosed`)
        (set `self.IsDoorClosed` false)
        (`GameplayStatics.PlaySoundAtLocation` "/Game/Sounds/Misc/OpenDoor.OpenDoor" _returnvalue (struct) 1.0 1.0 0.0 null null null null)
        (set `self.DotProduct` (`KismetMathLibrary.Dot_VectorVector` (`KismetMathLibrary.Normal` (- (`self.K2_GetActorLocation` self) (`self.K2_GetActorLocation` (`self.PlayerRef`)))) (`self.GetActorForwardVector` self)))
        (bind (_direction _alpha) (`Timeline|Timeline` :!label _label)
          (:`Update`
            (`SceneComponent.K2_SetRelativeRotation` (`self.StaticMesh1`) (`KismetMathLibrary.MakeRotator` 0.0 0.0 (`KismetMathLibrary.Lerp` 0.0 (select `bool` (>= (`self.DotProduct`) 0.0) :`false` -90.0 :`true` 90.0) _alpha)) false false)
            (`SceneComponent.K2_SetRelativeRotation` (`self.StaticMesh2`) (`KismetMathLibrary.MakeRotator` 0.0 0.0 (`KismetMathLibrary.Lerp` -180.0 (select `bool` (>= (`self.DotProduct`) 0.0) :`false` -90.0 :`true` -270.0) _alpha)) false false)))
        (else
          (set `self.IsDoorClosed` true)
          (`GameplayStatics.PlaySoundAtLocation` "/Game/Sounds/Misc/CloseDoor.CloseDoor" _returnvalue (struct) 1.0 1.0 0.0 null null null null)
          (goto _label :!via `Reverse`))))))

(event `/Game/Blueprints/Interface/BPI_Door.PickUpkey`
  (set `self.HasKey?` true))

(event `self.Box1.OnComponentBeginOverlap`
  (params (OverlappedComponent :type "PrimitiveComponent Object Reference") (OtherActor :type "Actor Object Reference") (OtherComp :type "PrimitiveComponent Object Reference") (OtherBodyIndex :type Integer) (bFromSweep :type Boolean) (SweepResult :type "HitResult Structure (by ref)"))
  (cast `/Game/Blueprints/PlayerCharacter/Level1/L1_Character` OtherActor)
  (`SceneComponent.SetVisibility` (`self.Widget`) true false))

(event `self.Box1.OnComponentEndOverlap`
  (params (OverlappedComponent :type "PrimitiveComponent Object Reference") (OtherActor :type "Actor Object Reference") (OtherComp :type "PrimitiveComponent Object Reference") (OtherBodyIndex :type Integer))
  (bind _opendoorwidget (`self.OpenDoorWidget`))
  (cast `/Game/Blueprints/PlayerCharacter/Level1/L1_Character` OtherActor)
  (`SceneComponent.SetVisibility` (`self.Widget`) false false)
  (if (`self.Tried to open door`)
    (`/Engine/EditorBlueprintResources/StandardMacros.IsValid` _opendoorwidget
      (:`Is Valid`
        _)
      (:`Is Not Valid`
        (bind _returnvalue (`|CreateWidget` "/Game/Widgets/OpenDoor_Widget.OpenDoor_Widget_C"))
        (bind _output_get (set `self.OpenDoorWidget` _returnvalue))))
    (`Widget.RemoveFromParent` _opendoorwidget)
    (`Widget.RemoveFromParent` _output_get)
    (set `self.Tried to open door` false)
    (set `self.DoorWidgetPrinted` false)))

(event `self.Box.OnComponentBeginOverlap`
  (params (OverlappedComponent :type "PrimitiveComponent Object Reference") (OtherActor :type "Actor Object Reference") (OtherComp :type "PrimitiveComponent Object Reference") (OtherBodyIndex :type Integer) (bFromSweep :type Boolean) (SweepResult :type "HitResult Structure (by ref)"))
  ;[1 1 1] Monster part
)

(event `self.Box.OnComponentEndOverlap`
  (params (OverlappedComponent :type "PrimitiveComponent Object Reference") (OtherActor :type "Actor Object Reference") (OtherComp :type "PrimitiveComponent Object Reference") (OtherBodyIndex :type Integer))
  ;[1 1 1] Monster part
)

(fn `UserConstructionScript`
  (`parent.UserConstructionScript`))