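; BP_LockedForveverDoor_Door is a permanently locked door that tells the player it cannot be used.
; Entering its WrongBox trigger plays a 2D locked-door sound, then creates, stores and displays a WrongDoorPopUp_Widget.
; Leaving the trigger removes the stored popup, first creating one if the reference is invalid.
; The overlap events do not check which actor triggers them, and the door has no opening logic.
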(event `self.Wrong box.OnComponentBeginOverlap`
  (params (OverlappedComponent :type "PrimitiveComponent Object Reference") (OtherActor :type "Actor Object Reference") (OtherComp :type "PrimitiveComponent Object Reference") (OtherBodyIndex :type Integer) (bFromSweep :type Boolean) (SweepResult :type "HitResult Structure (by ref)"))
  (`GameplayStatics.PlaySound2D` "/Game/Sounds/Mechanics/doorLocked.doorLocked" 1.0 1.0 0.0 null null)
  (bind _returnvalue (`|CreateWidget` "/Game/Widgets/WrongDoorPopUp_Widget.WrongDoorPopUp_Widget_C"))
  (bind _output_get (set `self.WrongDoorRef` _returnvalue))
  (`UserWidget.AddToViewport` _output_get 0))

(event `self.Wrong box.OnComponentEndOverlap`
  (params (OverlappedComponent :type "PrimitiveComponent Object Reference") (OtherActor :type "Actor Object Reference") (OtherComp :type "PrimitiveComponent Object Reference") (OtherBodyIndex :type Integer))
  (bind _wrongdoorref (`self.WrongDoorRef`))
  (`/Engine/EditorBlueprintResources/StandardMacros.IsValid` _wrongdoorref
    (:`Is Valid`
      _)
    (:`Is Not Valid`
      (bind _returnvalue (`|CreateWidget` "/Game/Widgets/WrongDoorPopUp_Widget.WrongDoorPopUp_Widget_C"))
      (bind _output_get (set `self.WrongDoorRef` _returnvalue))))
  (`Widget.RemoveFromParent` _wrongdoorref)
  (`Widget.RemoveFromParent` _output_get))

(fn `UserConstructionScript`
  (`parent.UserConstructionScript`))