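; Study door actor that slams shut when something overlaps its trigger box, then acts as a locked door.
; Overlapping SlamBox plays the DoorClose timeline in reverse, driving the door's relative yaw through a lerp.
; A DoOnce on the timeline update plays the slam sound and enables overlap events on LockedBox.
; Later LockedBox overlaps play a locked-door sound, with no check on the overlapping actor.
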(event `self.SlamBox.OnComponentBeginOverlap`
  (params (OverlappedComponent :type "PrimitiveComponent Object Reference") (OtherActor :type "Actor Object Reference") (OtherComp :type "PrimitiveComponent Object Reference") (OtherBodyIndex :type Integer) (bFromSweep :type Boolean) (SweepResult :type "HitResult Structure (by ref)"))
  (bind (_direction _doorclose) (`Timeline|DoorClose` :!via `Reverse`)
    (:`Update`
      (`SceneComponent.K2_SetRelativeRotation` (`self.Door`) (`KismetMathLibrary.MakeRotator` 0.0 0.0 (`KismetMathLibrary.Lerp` 0.0 -90.0 _doorclose)) false false)
      (`/Engine/EditorBlueprintResources/StandardMacros.DoOnce` false
        (:`Completed`
          (`GameplayStatics.PlaySoundAtLocation` "/Game/Sounds/Misc/DoorSlam.DoorSlam" (`self.K2_GetActorLocation`) (struct) 1.0 1.0 0.0 null null null null)
          (set `PrimitiveComponent.bGenerateOverlapEvents` true (`self.LockedBox`)))))))

(event `self.LockedBox.OnComponentBeginOverlap`
  (params (OverlappedComponent :type "PrimitiveComponent Object Reference") (OtherActor :type "Actor Object Reference") (OtherComp :type "PrimitiveComponent Object Reference") (OtherBodyIndex :type Integer) (bFromSweep :type Boolean) (SweepResult :type "HitResult Structure (by ref)"))
  (`GameplayStatics.PlaySoundAtLocation` "/Game/Sounds/Mechanics/WavFiles/doorLocked.doorLocked" (`self.K2_GetActorLocation`) (struct) 1.0 1.0 0.0 null null null null))

(fn `UserConstructionScript`)