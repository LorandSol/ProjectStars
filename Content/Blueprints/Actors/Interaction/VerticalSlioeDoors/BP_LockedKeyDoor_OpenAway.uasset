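; Locked key door actor that serves as the game's win trigger when the player reaches it holding the key.
; A box overlap casts to L1_Character and checks HasKey, playing a locked sound if it is missing.
; With the key and the matching main hall objective, it pauses, swaps all widgets for the survived menu, shows the cursor and clears the objective.
; The door rotation timeline is never triggered, so the door does not open.
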(event `self.Box.OnComponentBeginOverlap`
  (params (OverlappedComponent :type "PrimitiveComponent Object Reference") (OtherActor :type "Actor Object Reference") (OtherComp :type "PrimitiveComponent Object Reference") (OtherBodyIndex :type Integer) (bFromSweep :type Boolean) (SweepResult :type "HitResult Structure (by ref)"))
  (bind _returnvalue (`GameplayStatics.GetPlayerController` 0))
  (bind _asl1_character (cast `/Game/Blueprints/PlayerCharacter/Level1/L1_Character` OtherActor))
  (if (`/Game/Blueprints/PlayerCharacter/Level1/L1_Character.HasKey` _asl1_character)
    (if (`/Game/Blueprints/PlayerCharacter/Level1/L1_Character.PlayerHasAnObjective` (`self.PlayerRef`))
      (if (`KismetStringLibrary.EqualEqual_StrStr` (`/Game/Blueprints/PlayerCharacter/Level1/L1_Character.CurrentObjective` (`self.PlayerRef`)) "Test if this key works in the main hall")
        (`GameplayStatics.SetGamePaused` true)
        (`WidgetLayoutLibrary.RemoveAllWidgets`)
        (bind _returnvalue_2 (`|CreateWidget` "/Game/Widgets/MenuYouSurvivedWidget.MenuYouSurvivedWidget_C" _returnvalue))
        (`UserWidget.AddToViewport` _returnvalue_2 0)
        (set `PlayerController.bShowMouseCursor` true _returnvalue)
        (set `/Game/Blueprints/PlayerCharacter/Level1/L1_Character.PlayerHasAnObjective` false (`self.PlayerRef`))))
    (else
      (`GameplayStatics.PlaySound2D` "/Game/Sounds/Mechanics/WavFiles/doorLocked.doorLocked" 1.0 1.0 0.0 null null))))

(fn `UserConstructionScript`
  (`parent.UserConstructionScript`))