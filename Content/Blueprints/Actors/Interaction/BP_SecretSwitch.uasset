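; Secret switch actor, a picture frame that slides a referenced bookshelf aside when interacted with.
; Interact runs a Timeline that lerps the shelf by MoveObject along X or Y, chosen by Yaxis, and sets IsOpen to block reuse.
; That Timeline's updates drive a second one that tilts the frame.
; A DoOnce plays both slide sounds, clears the custom-depth highlight and disables the sphere's overlap events.
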(event `self.ReceiveBeginPlay`
  (`parent.ReceiveBeginPlay`))

(event `/Game/Blueprints/Interface/BPI_Interaction.Interact`
  (bind _yaxis (`self.Yaxis`))
  (bind _staticmesh (`self.StaticMesh`))
  (bind _staticmeshcomponent (`StaticMeshActor.StaticMeshComponent` (`self.BookShelf`)))
  (bind (_returnvalue_x _returnvalue_y _returnvalue_z) (`KismetMathLibrary.BreakVector` (`SceneComponent.K2_GetComponentLocation` _staticmeshcomponent)))
  ;[1 1 1] Moves static mesh (make sure static mesh is set to movable)
  (`/Engine/EditorBlueprintResources/StandardMacros.IsValid` (`self.BookShelf`) ; makes sure the reference is valid
    (:`Is Valid`
      (if (not (`self.isOpen`))
        (bind _output_get (set `self.MoveObject` (+ (`self.MoveObject`) (select `bool` _yaxis :`false` _returnvalue_x :`true` _returnvalue_y))))
        (bind (_direction _alpha) (`Timeline|Timeline`) ; creates a small animation so the object doesn't snap to position
          (:`Update`
            (if (`self.Yaxis`)
              (bind _returnvalue (`KismetMathLibrary.Lerp` (select `bool` _yaxis :`false` _returnvalue_x :`true` _returnvalue_y) _output_get _alpha))
              (`SceneComponent.K2_SetRelativeLocation` _staticmeshcomponent (`KismetMathLibrary.MakeVector` _returnvalue_x _returnvalue _returnvalue_z) false false)
              (else
                (`SceneComponent.K2_SetRelativeLocation` _staticmeshcomponent (`KismetMathLibrary.MakeVector` _returnvalue _returnvalue_y _returnvalue_z) false false)))
            (set `self.isOpen` true)
            (bind (_direction_2 _alpha_2) (`Timeline|PictureFrame`)
              (:`Update`
                (`SceneComponent.K2_SetRelativeRotation` _staticmesh (`KismetMathLibrary.MakeRotator` 90.0 (`KismetMathLibrary.Lerp` 0.0 20.0 _alpha_2)) false false)
                (`/Engine/EditorBlueprintResources/StandardMacros.DoOnce` false
                  (:`Completed`
                    (`GameplayStatics.PlaySoundAtLocation` "/Game/Sounds/Misc/PaintingSlide.PaintingSlide" (`SceneComponent.K2_GetComponentLocation` _staticmesh) (struct) 1.0 1.0 0.0 null null null null)
                    (`GameplayStatics.PlaySoundAtLocation` "/Game/Sounds/Mechanics/FurnitureDrag.FurnitureDrag" (`SceneComponent.K2_GetComponentLocation` _staticmeshcomponent) (struct) 1.0 1.0 0.0 null null null null)
                    (`PrimitiveComponent.SetRenderCustomDepth` (`self.StaticMesh`) false)
                    (set `PrimitiveComponent.bGenerateOverlapEvents` false (`self.Sphere`))))))))))))

(fn `UserConstructionScript`
  (`parent.UserConstructionScript`))