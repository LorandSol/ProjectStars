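; Interactable door that swings open away from whoever opens it, either the player or an AI_Classic character.
; A dot product of the door's forward vector and the opener's direction picks the swing side for timeline-driven yaw.
; Interact's branch is fixed to true, so it only runs the opening path.
; AI box overlap opens the door without collision and blocks interaction; leaving reverses it, restoring both once closed.
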(event `self.Interact`
  (bind _returnvalue (`self.K2_GetActorLocation`))
  (if true
    (set `self.IsDoorClosed` false)
    (`GameplayStatics.PlaySoundAtLocation` "/Game/Sounds/Misc/CloseDoor.CloseDoor" _returnvalue (struct) 1.0 1.0 0.0 null null null null)
    (set `self.DotProduct` (`KismetMathLibrary.Dot_VectorVector` (`KismetMathLibrary.Normal` (- (`self.K2_GetActorLocation` self) (`self.K2_GetActorLocation` (`self.PlayerRef`)))) (`self.GetActorForwardVector` self)))
    (bind (_direction _alpha) (`Timeline|Timeline` :!label _label)
      (:`Update`
        (`SceneComponent.K2_SetRelativeRotation` (`self.StaticMesh1`) (`KismetMathLibrary.MakeRotator` 0.0 0.0 (`KismetMathLibrary.Lerp` 0.0 (select `bool` (>= (`self.DotProduct`) 0.0) :`false` 85.0 :`true` -85.0) _alpha)) false false)))
    (else
      (set `self.IsDoorClosed` (`self.IsDoorClosed`))
      (`GameplayStatics.PlaySoundAtLocation` "/Game/Sounds/Misc/OpenDoor.OpenDoor" _returnvalue (struct) 1.0 1.0 0.0 null null null null)
      (goto _label :!via `Reverse`))))

(event `self.Box.OnComponentBeginOverlap`
  (params (OverlappedComponent :type "PrimitiveComponent Object Reference") (OtherActor :type "Actor Object Reference") (OtherComp :type "PrimitiveComponent Object Reference") (OtherBodyIndex :type Integer) (bFromSweep :type Boolean) (SweepResult :type "HitResult Structure (by ref)"))
  (bind _asai_classic (cast `/Game/AI/Classic/AI_Classic` OtherActor))
  (set `self.canInteract` false)
  (if (`self.IsDoorClosed`)
    (set `self.IsDoorClosed` false)
    (set `self.DotProduct` (`KismetMathLibrary.Dot_VectorVector` (`KismetMathLibrary.Normal` (- (`self.K2_GetActorLocation` self) (`self.K2_GetActorLocation` _asai_classic))) (`self.GetActorForwardVector` self)))
    (bind (_direction _alpha) (`Timeline|Open Door AI` :!label _label_2)
      (:`Update`
        (`PrimitiveComponent.SetCollisionEnabled` (`self.StaticMesh1`) "NoCollision")
        (`SceneComponent.K2_SetRelativeRotation` (`self.StaticMesh1`) (`KismetMathLibrary.MakeRotator` 0.0 0.0 (`KismetMathLibrary.Lerp` 0.0 (select `bool` (>= (`self.DotProduct`) 0.0) :`false` 85.0 :`true` -85.0) _alpha)) false false))
      (:`Finished`
        (switch `ETimelineDirection` _direction
          (:`Backward`
            (`PrimitiveComponent.SetCollisionEnabled` (`self.StaticMesh1`) "QueryAndPhysics")
            (set `self.canInteract` true)))))))

(event `self.Box.OnComponentEndOverlap`
  (params (OverlappedComponent :type "PrimitiveComponent Object Reference") (OtherActor :type "Actor Object Reference") (OtherComp :type "PrimitiveComponent Object Reference") (OtherBodyIndex :type Integer))
  (cast `/Game/AI/Classic/AI_Classic` OtherActor)
  (if (not (`self.isDoorClosed`))
    (set `self.IsDoorClosed` true)
    (goto _label_2 :!via `ReverseFromEnd`)))

(fn `UserConstructionScript`
  (`parent.UserConstructionScript`))