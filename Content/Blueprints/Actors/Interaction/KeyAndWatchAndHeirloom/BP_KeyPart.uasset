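; BP_KeyPart is an interactable pickup for one piece of a two-part key.
; On Interact it adds its part value to the key total stored on L1_Character.
; A total of one or two updates the collected-count text, plays an objective sound and a second sound at world origin, then destroys the actor.
; Any other total leaves the pickup in place.
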(event `/Game/Blueprints/Interface/BPI_Interaction.Interact`
  (bind _asl1_character (cast `/Game/Blueprints/PlayerCharacter/Level1/L1_Character` (`GameplayStatics.GetPlayerCharacter` 0)))
  (bind _output_get (set `/Game/Blueprints/PlayerCharacter/Level1/L1_Character.KeyPart_TotalAmount` (+ (`/Game/Blueprints/PlayerCharacter/Level1/L1_Character.KeyPart_TotalAmount` _asl1_character) (`self.KeyPart_Single`)) _asl1_character))
  (if (== _output_get 1)
    (set `/Game/Blueprints/PlayerCharacter/Level1/L1_Character.KeysCollectedText` "1 of 2" _asl1_character)
    (`GameplayStatics.PlaySound2D` "/Game/Sounds/Mechanics/WavFiles/objective2.objective2" 1.0 1.0 0.0 null null :!label _label)
    (`GameplayStatics.PlaySoundAtLocation` "/Game/Sounds/Jumpscares/ISeeYou.ISeeYou" (0.0 0.0 0.0) (struct) 1.0 1.0 0.0 null null null null)
    (`self.K2_DestroyActor`)
    (elif (== _output_get 2)
      (set `/Game/Blueprints/PlayerCharacter/Level1/L1_Character.KeysCollectedText` "2 of 2" _asl1_character)
      (goto _label))))

(fn `UserConstructionScript`)