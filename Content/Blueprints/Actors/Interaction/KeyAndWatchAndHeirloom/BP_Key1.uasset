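; BP_Key1 is an interactable key pickup that gives the player a key and assigns a new objective.
; Interact sets HasKey on the L1_Character and calls PickUpkeyMessage on two referenced doors.
; It then clears and resets the player's objective, sets CurrentObjective, plays two 2D sounds and shows an objective popup widget.
; The actor destroys itself afterwards.
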(event `self.Interact`
  (bind _asl1_character (cast `/Game/Blueprints/PlayerCharacter/Level1/L1_Character` (`GameplayStatics.GetPlayerCharacter` 0)))
  (bind _output_get (set `self.CharVar` _asl1_character))
  (set `/Game/Blueprints/PlayerCharacter/Level1/L1_Character.HasKey` true _output_get)
  (message `/Game/Blueprints/Interface/BPI_Door.PickUpkey` (`self.Door`))
  (message `/Game/Blueprints/Interface/BPI_Door.PickUpkey` (`self.Door2`))
  (set `/Game/Blueprints/PlayerCharacter/Level1/L1_Character.PlayerHasAnObjective` false _asl1_character)
  (if (not (`/Game/Blueprints/PlayerCharacter/Level1/L1_Character.PlayerHasAnObjective` _asl1_character))
    (set `/Game/Blueprints/PlayerCharacter/Level1/L1_Character.CurrentObjective` (`self.Objective`) _asl1_character)
    (set `/Game/Blueprints/PlayerCharacter/Level1/L1_Character.PlayerHasAnObjective` true _asl1_character)
    (`GameplayStatics.PlaySound2D` "/Game/Sounds/Mechanics/WavFiles/objective2.objective2" 1.0 1.0 0.0 null null)
    (bind _returnvalue (`|CreateWidget` "/Game/Widgets/Objectives/ObjectivePopUp.ObjectivePopUp_C"))
    (bind _output_get_2 (set `self.ObjectivePopUp` _returnvalue))
    (`UserWidget.AddToViewport` _output_get_2 0)
    (`GameplayStatics.PlaySound2D` "/Game/Sounds/Mechanics/WavFiles/CheckScribble2.CheckScribble2" 1.0 1.0 0.0 null null)
    (`self.K2_DestroyActor`)))

(fn `UserConstructionScript`
  (`parent.UserConstructionScript`))