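; BP_Heirloom is an interactable heirloom pickup for the L1 character.
; On Interact it flags the character as holding the heirloom and clears its active-objective flag, so the following check passes.
; It then assigns its own objective as the current one, sets the flag again and shows an objective popup widget.
; Finally it plays scribble and special-item sounds and destroys itself.
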(event `/Game/Blueprints/Interface/BPI_Interaction.Interact`
  (bind _asl1_character (cast `/Game/Blueprints/PlayerCharacter/Level1/L1_Character` (`GameplayStatics.GetPlayerCharacter` 0)))
  (bind _output_get (set `self.As L1 Character` _asl1_character))
  (set `/Game/Blueprints/PlayerCharacter/Level1/L1_Character.HasHeirloom` true _output_get)
  (set `/Game/Blueprints/PlayerCharacter/Level1/L1_Character.PlayerHasAnObjective` false _asl1_character)
  (if (not (`/Game/Blueprints/PlayerCharacter/Level1/L1_Character.PlayerHasAnObjective` _asl1_character))
    (set `/Game/Blueprints/PlayerCharacter/Level1/L1_Character.CurrentObjective` (`self.Objective`) _asl1_character)
    (set `/Game/Blueprints/PlayerCharacter/Level1/L1_Character.PlayerHasAnObjective` true _asl1_character)
    (bind _returnvalue (`|CreateWidget` "/Game/Widgets/Objectives/ObjectivePopUp.ObjectivePopUp_C"))
    (bind _output_get_2 (set `self.ObjectivePopUp` _returnvalue))
    (`UserWidget.AddToViewport` _output_get_2 0)
    (`GameplayStatics.PlaySound2D` "/Game/Sounds/Mechanics/WavFiles/CheckScribble2.CheckScribble2" 1.0 1.0 0.0 null null)
    (`GameplayStatics.PlaySound2D` "/Game/Sounds/Mechanics/SpecialItem.SpecialItem" 1.0 1.0 0.0 null null)
    (`self.K2_DestroyActor`)))

(fn `UserConstructionScript`
  (`parent.UserConstructionScript`))