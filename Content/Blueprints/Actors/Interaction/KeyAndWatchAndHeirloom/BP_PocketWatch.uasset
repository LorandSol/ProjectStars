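; Pocket watch pickup that grants the player character the watch and the ability to time travel.
; Interact always flags the watch as held, but only plays the objective sound, enables time travel and destroys the actor when the player has no objective.
; A box overlap toggles the widget, while a sphere overlap toggles a custom-depth highlight for the player.
; The time travel prompt widget creation is unconnected and never runs.
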(event `self.Interact`
  (bind _asl1_character (cast `/Game/Blueprints/PlayerCharacter/Level1/L1_Character` (`GameplayStatics.GetPlayerCharacter` 0)))
  (bind _output_get (set `self.CharVar` _asl1_character))
  (set `/Game/Blueprints/PlayerCharacter/Level1/L1_Character.HasPocketWatch` true _output_get)
  (if (not (`/Game/Blueprints/PlayerCharacter/Level1/L1_Character.PlayerHasAnObjective` _asl1_character))
    (`GameplayStatics.PlaySound2D` "/Game/Sounds/Mechanics/objective2.objective2" 1.0 1.0 0.0 null null)
    (set `/Game/Blueprints/PlayerCharacter/Level1/L1_Character.canTimeTravel?` true (`self.CharVar`))
    (set `self.PickedUp` true)
    (`self.K2_DestroyActor`)))

(event `self.Box.OnComponentBeginOverlap`
  (params (OverlappedComponent :type "PrimitiveComponent Object Reference") (OtherActor :type "Actor Object Reference") (OtherComp :type "PrimitiveComponent Object Reference") (OtherBodyIndex :type Integer) (bFromSweep :type Boolean) (SweepResult :type "HitResult Structure (by ref)"))
  (`SceneComponent.SetVisibility` (`self.Widget`) true false))

(event `self.Box.OnComponentEndOverlap`
  (params (OverlappedComponent :type "PrimitiveComponent Object Reference") (OtherActor :type "Actor Object Reference") (OtherComp :type "PrimitiveComponent Object Reference") (OtherBodyIndex :type Integer))
  (`SceneComponent.SetVisibility` (`self.Widget`) false false))

(event `self.Sphere.OnComponentBeginOverlap`
  (params (OverlappedComponent :type "PrimitiveComponent Object Reference") (OtherActor :type "Actor Object Reference") (OtherComp :type "PrimitiveComponent Object Reference") (OtherBodyIndex :type Integer) (bFromSweep :type Boolean) (SweepResult :type "HitResult Structure (by ref)"))
  (cast `/Game/Blueprints/PlayerCharacter/Level1/L1_Character` OtherActor)
  (`PrimitiveComponent.SetRenderCustomDepth` (`self.Pocket`) true))

(event `self.Sphere.OnComponentEndOverlap`
  (params (OverlappedComponent :type "PrimitiveComponent Object Reference") (OtherActor :type "Actor Object Reference") (OtherComp :type "PrimitiveComponent Object Reference") (OtherBodyIndex :type Integer))
  (cast `/Game/Blueprints/PlayerCharacter/Level1/L1_Character` OtherActor)
  (`PrimitiveComponent.SetRenderCustomDepth` (`self.Pocket`) false))

(fn `UserConstructionScript`
  (`parent.UserConstructionScript`))