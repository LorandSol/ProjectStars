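; One-shot jumpscare trigger that briefly shows an AI_Classic enemy and knocks out the player's flashlight.
; The first Box overlap by any actor spawns the AI at a hard-coded transform, flickers the cached L1_Character's spotlight, then quickly destroys the AI.
; The light stays off and locked for a few seconds.
; It then returns to normal, a voice cue plays and time travel is enabled on the character.
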(event `self.ReceiveBeginPlay`
  (bind _asl1_character (cast `/Game/Blueprints/PlayerCharacter/Level1/L1_Character` (`GameplayStatics.GetPlayerCharacter` 0)))
  (set `self.CharVar` _asl1_character))

(event `self.Box.OnComponentBeginOverlap`
  (params (OverlappedComponent :type "PrimitiveComponent Object Reference") (OtherActor :type "Actor Object Reference") (OtherComp :type "PrimitiveComponent Object Reference") (OtherBodyIndex :type Integer) (bFromSweep :type Boolean) (SweepResult :type "HitResult Structure (by ref)"))
  (bind _charvar (`self.CharVar`))
  (bind _spotlight1 (`/Game/Blueprints/PlayerCharacter/Level1/L1_Character.SpotLight1` _charvar))
  (`/Engine/EditorBlueprintResources/StandardMacros.DoOnce` false
    (:`Completed`
      (bind _returnvalue (`|SpawnActorFromClass` "/Game/AI/Classic/AI_Classic.AI_Classic_C" (`KismetMathLibrary.MakeTransform` (1660.0 -1340.0 1200.0) (struct :`Pitch` 180.0)) "AlwaysSpawn" "MultiplyWithRoot" null null))
      (`LightComponent.SetLightFunctionMaterial` _spotlight1 "/Game/Props/Materials/LightFlicker.LightFlicker")
      (`KismetSystemLibrary.Delay` 0.2)
      (`self.K2_DestroyActor` _returnvalue)
      (`SceneComponent.SetVisibility` _spotlight1 false false)
      (set `/Game/Blueprints/PlayerCharacter/Level1/L1_Character.CanToggleFlashlight` false _charvar)
      (`KismetSystemLibrary.Delay` 4.0)
      (`SceneComponent.SetVisibility` _spotlight1 true false)
      (set `/Game/Blueprints/PlayerCharacter/Level1/L1_Character.CanToggleFlashlight` true _charvar)
      (`LightComponent.SetLightFunctionMaterial` _spotlight1 "/Game/Props/Materials/LightNormal.LightNormal")
      (`GameplayStatics.PlaySound2D` "/Game/Sounds/Jumpscares/I_See_You2.I_See_You2" 1.0 1.0 0.0 null null)
      (set `/Game/Blueprints/PlayerCharacter/Level1/L1_Character.canTimeTravel?` true _charvar))))

(fn `UserConstructionScript`)