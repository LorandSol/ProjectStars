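; Trigger actor that starts a chase sequence, apparently in the past timeline, when its box is first overlapped.
; BeginPlay caches the player as L1_Character.
; The overlap fires two one-shot branches without filtering the overlapping actor.
; One spawns an AI_Classic at a hardcoded transform, applies a flicker light function to the player's spotlight, plays chase audio and disables time travel; the other spawns BP_TeleportPresent at a fixed location.
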(event `self.ReceiveBeginPlay`
  (bind _asl1_character (cast `/Game/Blueprints/PlayerCharacter/Level1/L1_Character` (`GameplayStatics.GetPlayerCharacter` 0)))
  (set `self.CharVar` _asl1_character))

(event `self.Box.OnComponentBeginOverlap`
  (params (OverlappedComponent :type "PrimitiveComponent Object Reference") (OtherActor :type "Actor Object Reference") (OtherComp :type "PrimitiveComponent Object Reference") (OtherBodyIndex :type Integer) (bFromSweep :type Boolean) (SweepResult :type "HitResult Structure (by ref)"))
  (bind _charvar (`self.CharVar`))
  (`|ExecutionSequence`
    (:`then_0`
      (`/Engine/EditorBlueprintResources/StandardMacros.DoOnce` false
        (:`Completed`
          (`|SpawnActorFromClass` "/Game/AI/Classic/AI_Classic.AI_Classic_C" (`KismetMathLibrary.MakeTransform` (1730.0 -3250.0 1200.0) (struct :`Yaw` 90.0)) "AlwaysSpawn" "MultiplyWithRoot" null null)
          (`LightComponent.SetLightFunctionMaterial` (`/Game/Blueprints/PlayerCharacter/Level1/L1_Character.SpotLight1` _charvar) "/Game/Props/Materials/LightFlicker.LightFlicker")
          (`GameplayStatics.SpawnSound2D` "/Game/Sounds/Mechanics/Chase.Chase" 1.0 1.0 0.0 null)
          (set `/Game/Blueprints/PlayerCharacter/Level1/L1_Character.canTimeTravel?` false _charvar))))
    (:`then_1`
      (`/Engine/EditorBlueprintResources/StandardMacros.DoOnce` false
        (:`Completed`
          (`|SpawnActorFromClass` "/Game/Blueprints/Actors/Objectives/BP_TeleportPresent.BP_TeleportPresent_C" (`KismetMathLibrary.MakeTransform` (890.0 -910.0 1100.0)) "Undefined" "MultiplyWithRoot" null null))))))

(fn `UserConstructionScript`)