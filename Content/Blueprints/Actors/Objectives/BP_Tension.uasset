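; BP_Tension is an objective actor that travels along a spline path in the level and then destroys itself.
; On BeginPlay it finds a BP_SplinePath actor and plays a timeline scaled by TimeToComplete.
; Each update maps the timeline alpha to distance along the spline, setting the actor's location and rotation.
; A Delay chained to the update destroys it ten seconds after movement starts, independent of TimeToComplete.
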(event `self.ReceiveBeginPlay`
  (bind _returnvalue (`GameplayStatics.GetActorOfClass` "/Game/Blueprints/Actors/Objectives/BP_SplinePath.BP_SplinePath_C"))
  (set `self.SplineRef` _returnvalue)
  (`self.MoveObject`))

(event `MoveObject`
  (bind _spline (`/Game/Blueprints/Actors/Objectives/BP_SplinePath.Spline` (`self.SplineRef`)))
  (`TimelineComponent.SetPlayRate` (`self.TensionTime`) (/ 1.0 (`self.TimeToComplete`)))
  (bind (_direction _movetension) (`Timeline|TensionTime`)
    (:`Update`
      (bind _returnvalue (`KismetMathLibrary.Lerp` 0.0 (`SplineComponent.GetSplineLength` (`/Game/Blueprints/Actors/Objectives/BP_SplinePath.Spline` (`self.SplineRef`))) _movetension))
      (`self.K2_SetActorTransform` (`KismetMathLibrary.MakeTransform` (`SplineComponent.GetLocationAtDistanceAlongSpline` _spline _returnvalue "World") (`SplineComponent.GetRotationAtDistanceAlongSpline` _spline _returnvalue "World")))
      (`KismetSystemLibrary.Delay` 10.0)
      (`self.K2_DestroyActor`))))

(fn `UserConstructionScript`)