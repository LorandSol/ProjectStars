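; BP_TeleportPresent is an objective trigger that moves the player from the past to the present level.
; It caches the L1_Character on BeginPlay, and the first overlap on its Box plays a time-travel sound and drops the character a fixed distance below its camera's location.
; It then sets the character's PresentLevel flag and removes the past tint widget from the screen.
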(event `self.ReceiveBeginPlay`
  (bind _asl1_character (cast `/Game/Blueprints/PlayerCharacter/Level1/L1_Character` (`GameplayStatics.GetPlayerCharacter` 0)))
  (set `self.CharVar` _asl1_character))

(event `self.Box.OnComponentBeginOverlap`
  (params (OverlappedComponent :type "PrimitiveComponent Object Reference") (OtherActor :type "Actor Object Reference") (OtherComp :type "PrimitiveComponent Object Reference") (OtherBodyIndex :type Integer) (bFromSweep :type Boolean) (SweepResult :type "HitResult Structure (by ref)"))
  (bind _charvar (`self.CharVar`))
  (bind (_returnvalue_x _returnvalue_y _returnvalue_z) (`KismetMathLibrary.BreakVector` (`SceneComponent.K2_GetComponentLocation` (`/Game/Blueprints/PlayerCharacter/Level1/L1_Character.Camera` _charvar))))
  (`/Engine/EditorBlueprintResources/StandardMacros.DoOnce` false
    (:`Completed`
      (`GameplayStatics.PlaySoundAtLocation` "/Game/Sounds/Mechanics/TimeTravel.TimeTravel" (0.0 0.0 0.0) (struct) 1.0 1.0 0.0 null null null null)
      (`self.K2_SetActorLocation` _charvar (`KismetMathLibrary.MakeVector` _returnvalue_x _returnvalue_y (- _returnvalue_z 1100.0)) false false)
      (set `/Game/Blueprints/PlayerCharacter/Level1/L1_Character.PresentLevel` true _charvar)
      (`Widget.RemoveFromParent` (`/Game/Blueprints/PlayerCharacter/Level1/L1_Character.PastTintRef` _charvar)))))

(fn `UserConstructionScript`)