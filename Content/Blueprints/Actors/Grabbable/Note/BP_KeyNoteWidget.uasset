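; BP_KeyNoteWidget is an interactable note actor that the player can read and put down.
; Interact toggles reading: it hides the note, adds the KeyNoteWritten widget to the viewport and plays a paper sound, then reverses the visuals on the next call.
; While the note is held, character movement and player controller input are disabled.
; A sphere overlap with L1_Character toggles custom depth on the note mesh for highlighting.
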(event `self.Interact`
  (if (not (`self.HoldingNote?`))
    (set `self.HoldingNote?` true)
    (`self.SetActorHiddenInGame` (`ActorComponent.GetOwner` (`self.TestNote`)) true)
    (bind _returnvalue (`|CreateWidget` "/Game/Blueprints/Actors/Grabbable/Note/KeyNoteWritten_widget.KeyNoteWritten_widget_C"))
    (bind _output_get (set `self.NewVar` _returnvalue))
    (`UserWidget.AddToViewport` _output_get 0)
    (bind _asl1_character (cast `/Game/Blueprints/PlayerCharacter/Level1/L1_Character` (`GameplayStatics.GetPlayerCharacter` 0)))
    (`CharacterMovementComponent.DisableMovement` (`Character.CharacterMovement` _asl1_character))
    (bind _ashg_player_controller (cast `/Game/Blueprints/PlayerCharacter/HG_PlayerController` (`GameplayStatics.GetPlayerController` 0)))
    (`self.DisableInput` _ashg_player_controller _ashg_player_controller)
    (`GameplayStatics.PlaySound2D` "/Game/Sounds/Mechanics/Paper.Paper" 1.0 1.0 0.0 null null)
    (else
      (set `self.HoldingNote?` false)
      (`Widget.RemoveFromParent` (`self.NewVar`))
      (`self.SetActorHiddenInGame` (`ActorComponent.GetOwner` (`self.TestNote`)) false)
      (bind _asl1_character_2 (cast `/Game/Blueprints/PlayerCharacter/Level1/L1_Character` (`GameplayStatics.GetPlayerCharacter` 0)))
      (`CharacterMovementComponent.SetMovementMode` (`Character.CharacterMovement` _asl1_character_2) "MOVE_Walking" 0)
      (bind _ashg_player_controller_2 (cast `/Game/Blueprints/PlayerCharacter/HG_PlayerController` (`GameplayStatics.GetPlayerController` 0)))
      (`self.EnableInput` _ashg_player_controller_2 _ashg_player_controller_2))))

(event `self.Sphere.OnComponentBeginOverlap`
  (params (OverlappedComponent :type "PrimitiveComponent Object Reference") (OtherActor :type "Actor Object Reference") (OtherComp :type "PrimitiveComponent Object Reference") (OtherBodyIndex :type Integer) (bFromSweep :type Boolean) (SweepResult :type "HitResult Structure (by ref)"))
  (cast `/Game/Blueprints/PlayerCharacter/Level1/L1_Character` OtherActor)
  (`PrimitiveComponent.SetRenderCustomDepth` (`self.TestNote`) true))

(event `self.Sphere.OnComponentEndOverlap`
  (params (OverlappedComponent :type "PrimitiveComponent Object Reference") (OtherActor :type "Actor Object Reference") (OtherComp :type "PrimitiveComponent Object Reference") (OtherBodyIndex :type Integer))
  (cast `/Game/Blueprints/PlayerCharacter/Level1/L1_Character` OtherActor)
  (`PrimitiveComponent.SetRenderCustomDepth` (`self.TestNote`) false))

(fn `UserConstructionScript`)