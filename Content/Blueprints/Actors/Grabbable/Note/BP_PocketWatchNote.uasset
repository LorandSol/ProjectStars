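; BP_PocketWatchNote is an interactable note actor that toggles a readable pocket watch note on screen.
; The first Interact hides the actor, shows the Note2_Widget_Pocket widget with a paper sound, disables player movement and input, blocks the pause menu and pauses the game.
; The next Interact removes the widget, unhides the actor and restores movement, input and pausing.
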(event `/Game/Blueprints/Interface/BPI_Interaction.Interact`
  (if (not (`self.HoldingNote?`))
    (set `self.HoldingNote?` true)
    (`self.SetActorHiddenInGame` (`ActorComponent.GetOwner` (`self.StaticMesh`)) true)
    (bind _returnvalue (`|CreateWidget` "/Game/Blueprints/Actors/Grabbable/Note/Note2_Widget_Pocket.Note2_Widget_Pocket_C"))
    (bind _output_get (set `self.NoteWidgetRef` _returnvalue))
    (`UserWidget.AddToViewport` _output_get 0)
    (bind _asl1_character (cast `/Game/Blueprints/PlayerCharacter/Level1/L1_Character` (`GameplayStatics.GetPlayerCharacter` 0)))
    (`CharacterMovementComponent.DisableMovement` (`Character.CharacterMovement` _asl1_character))
    (bind _ashg_player_controller (cast `/Game/Blueprints/PlayerCharacter/HG_PlayerController` (`GameplayStatics.GetPlayerController` 0)))
    (`self.DisableInput` _ashg_player_controller _ashg_player_controller)
    (set `/Game/Blueprints/PlayerCharacter/Level1/L1_Character.CantPauseGame` true _asl1_character)
    (`GameplayStatics.PlaySound2D` "/Game/Sounds/Mechanics/Paper.Paper" 1.0 1.0 0.0 null null)
    (`GameplayStatics.SetGamePaused` true)
    (else
      (set `self.HoldingNote?` false)
      (`Widget.RemoveFromParent` (`self.NoteWidgetRef`))
      (`self.SetActorHiddenInGame` (`ActorComponent.GetOwner` (`self.StaticMesh`)) false)
      (bind _asl1_character_2 (cast `/Game/Blueprints/PlayerCharacter/Level1/L1_Character` (`GameplayStatics.GetPlayerCharacter` 0)))
      (`CharacterMovementComponent.SetMovementMode` (`Character.CharacterMovement` _asl1_character_2) "MOVE_Walking" 0)
      (bind _ashg_player_controller_2 (cast `/Game/Blueprints/PlayerCharacter/HG_PlayerController` (`GameplayStatics.GetPlayerController` 0)))
      (`self.EnableInput` _ashg_player_controller_2 _ashg_player_controller_2)
      (set `/Game/Blueprints/PlayerCharacter/Level1/L1_Character.CantPauseGame` false _asl1_character)
      (`GameplayStatics.SetGamePaused` false))))

(fn `UserConstructionScript`)