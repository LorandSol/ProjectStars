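; Grabbable map pickup that gives the player possession of the map.
; On Interact it casts the player character to L1_Character, sets PlayerHasMap and destroys itself.
; A Sphere overlap toggles custom depth rendering on the TestNote component while an L1_Character is in range, flagging it for highlighting.
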(event `/Game/Blueprints/Interface/BPI_Interaction.Interact`
  (bind _asl1_character (cast `/Game/Blueprints/PlayerCharacter/Level1/L1_Character` (`GameplayStatics.GetPlayerCharacter` 0)))
  (set `self.As L1 Character` _asl1_character)
  (set `/Game/Blueprints/PlayerCharacter/Level1/L1_Character.PlayerHasMap` true (`self.As L1 Character`))
  (`self.K2_DestroyActor`))

(event `self.Sphere.OnComponentBeginOverlap`
  (params (OverlappedComponent :type "PrimitiveComponent Object Reference") (OtherActor :type "Actor Object Reference") (OtherComp :type "PrimitiveComponent Object Reference") (OtherBodyIndex :type Integer) (bFromSweep :type Boolean) (SweepResult :type "HitResult Structure (by ref)"))
  (cast `/Game/Blueprints/PlayerCharacter/Level1/L1_Character` OtherActor)
  (`PrimitiveComponent.SetRenderCustomDepth` (`self.TestNote`) true))

(event `self.Sphere.OnComponentEndOverlap`
  (params (OverlappedComponent :type "PrimitiveComponent Object Reference") (OtherActor :type "Actor Object Reference") (OtherComp :type "PrimitiveComponent Object Reference") (OtherBodyIndex :type Integer))
  (cast `/Game/Blueprints/PlayerCharacter/Level1/L1_Character` OtherActor)
  (`PrimitiveComponent.SetRenderCustomDepth` (`self.TestNote`) false))

(fn `UserConstructionScript`)