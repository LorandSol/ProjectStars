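; World map component meant to show a map widget with the player's position marker, though most of its logic is disconnected.
; Only ShowMap is wired: it toggles widget visibility, input mode, player movement and controller input, playing a sound on opening.
; Initialization, toggling and marker updates are empty stubs.
; Unreachable nodes retain widget creation and corner-bound scaling of world location to map position, with X/Y axes swapped.
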(event `self.ReceiveBeginPlay`)

(event `InitializeMap`
  (params (Player :type "Character Object Reference")))

(event `OnPlayerMoved`)

(fn `ConvertLocationToMapLocation`
  (params (Location :type "Vector Structure"))
  (returns (Out :type "Vector2D Structure")))

(fn `GetMapHeight`
  (returns (Out :type "Float (double-precision)")))

(fn `GetMapWidth`
  (returns (Out :type "Float (double-precision)")))

(fn `LocationToMapPosition`
  (params (Location :type "Vector Structure") (WidgetSize :type "Vector2D Structure"))
  (returns (Out :type "Vector2D Structure")))

(fn `ShowMap`
  (params (`Show?` :type Boolean))
  (bind _returnvalue (`GameplayStatics.GetPlayerController` 0))
  (if (!= `Show?` (`self.Visible`))
    (bind _output_get (set `self.Visible` `Show?`))
    (if _output_get
      (`Widget.SetVisibility` (`self.MainRef`) "Visible")
      (`WidgetBlueprintLibrary.SetInputMode_GameAndUIEx` _returnvalue (`self.MainRef`) "DoNotLock" false)
      (`GameplayStatics.PlaySound2D` "/Game/Sounds/Mechanics/NoteUp.NoteUp" 1.0 1.0 0.0 null null)
      (`CharacterMovementComponent.DisableMovement` (`Character.CharacterMovement` (`self.Player`)))
      (bind _ashg_player_controller (cast `/Game/Blueprints/PlayerCharacter/HG_PlayerController` (`GameplayStatics.GetPlayerController` 0)))
      (`Actor.DisableInput` _ashg_player_controller _ashg_player_controller)
      (`self.UpdatePlayerPositionOnMap`)
      (return)
      (else
        (`Widget.SetVisibility` (`self.MainRef`) "Hidden")
        (`CharacterMovementComponent.SetMovementMode` (`Character.CharacterMovement` (`self.Player`)) "MOVE_Walking" 0)
        (bind _ashg_player_controller_2 (cast `/Game/Blueprints/PlayerCharacter/HG_PlayerController` (`GameplayStatics.GetPlayerController` 0)))
        (`Actor.EnableInput` _ashg_player_controller_2 _ashg_player_controller_2)
        (`WidgetBlueprintLibrary.SetInputMode_GameOnly` _returnvalue)
        (return)))
    (else
      (return))))

(fn `ToggleVisibility`)

(fn `UpdatePlayerPositionOnMap`)