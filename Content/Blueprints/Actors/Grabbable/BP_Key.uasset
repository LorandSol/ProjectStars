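; BP_Key is a key pickup that completes the player's "Find the key" objective when the L1_Character overlaps its Box.
; The overlap only acts while that objective is current, then flags the character as having the key.
; It replaces the current objective with its own Objective value, plays the Objective2 sound in 2D and destroys itself.
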(event `self.Box.OnComponentBeginOverlap`
  (params (OverlappedComponent :type "PrimitiveComponent Object Reference") (OtherActor :type "Actor Object Reference") (OtherComp :type "PrimitiveComponent Object Reference") (OtherBodyIndex :type Integer) (bFromSweep :type Boolean) (SweepResult :type "HitResult Structure (by ref)"))
  (bind _asl1_character (cast `/Game/Blueprints/PlayerCharacter/Level1/L1_Character` OtherActor))
  (if (`/Game/Blueprints/PlayerCharacter/Level1/L1_Character.PlayerHasAnObjective` _asl1_character)
    (if (`KismetStringLibrary.EqualEqual_StrStr` (`/Game/Blueprints/PlayerCharacter/Level1/L1_Character.CurrentObjective` _asl1_character) "Find the key")
      (set `/Game/Blueprints/PlayerCharacter/Level1/L1_Character.HasKey` true _asl1_character)
      (set `/Game/Blueprints/PlayerCharacter/Level1/L1_Character.PlayerHasAnObjective` false _asl1_character)
      (if (not (`/Game/Blueprints/PlayerCharacter/Level1/L1_Character.PlayerHasAnObjective` _asl1_character))
        (set `/Game/Blueprints/PlayerCharacter/Level1/L1_Character.CurrentObjective` (`self.Objective`) _asl1_character)
        (set `/Game/Blueprints/PlayerCharacter/Level1/L1_Character.PlayerHasAnObjective` true _asl1_character)
        (`GameplayStatics.PlaySound2D` "/Game/Sounds/Mechanics/objective2.objective2" 1.0 1.0 0.0 null null)
        (`self.K2_DestroyActor`)))))

(fn `UserConstructionScript`)