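; BP_AISpawner is a trigger volume that spawns an AI_Improved enemy and gives the player a new objective.
; When L1_Character enters the Box, it plays a roar at two locations, sets the "Find the master bedroom" objective and shows a popup with a scribble sound.
; Any end overlap destroys every BP_AISpawner in the level, with no check on which actor left.
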(event `self.Box.OnComponentBeginOverlap`
  (params (OverlappedComponent :type "PrimitiveComponent Object Reference") (OtherActor :type "Actor Object Reference") (OtherComp :type "PrimitiveComponent Object Reference") (OtherBodyIndex :type Integer) (bFromSweep :type Boolean) (SweepResult :type "HitResult Structure (by ref)"))
  (bind _as_l1_character (`self.As L1 Character`))
  (bind _asl1_character (cast `/Game/Blueprints/PlayerCharacter/Level1/L1_Character` OtherActor))
  (set `self.As L1 Character` _asl1_character)
  (`|SpawnActorFromClass` "/Game/AI/ImprovedAI/AI_Improved.AI_Improved_C" (`self.Spawn Transform`) "Undefined" "MultiplyWithRoot" null null)
  (`GameplayStatics.PlaySoundAtLocation` "/Game/Sounds/Jumpscares/DoTheRoar.DoTheRoar" (`self.Location_0`) (struct) 1.0 1.0 0.0 null null null null)
  (`GameplayStatics.PlaySoundAtLocation` "/Game/Sounds/Jumpscares/DoTheRoar.DoTheRoar" (`self.Location`) (struct) 1.0 1.0 0.0 null null null null)
  (set `/Game/Blueprints/PlayerCharacter/Level1/L1_Character.CurrentObjective` "Find the master bedroom" _as_l1_character)
  (set `/Game/Blueprints/PlayerCharacter/Level1/L1_Character.PlayerHasAnObjective` true _as_l1_character)
  (bind _returnvalue (`|CreateWidget` "/Game/Widgets/Objectives/ObjectivePopUp.ObjectivePopUp_C"))
  (bind _output_get (set `self.ObjectivePopUp` _returnvalue))
  (`UserWidget.AddToViewport` _output_get 0)
  (`GameplayStatics.PlaySound2D` "/Game/Sounds/Mechanics/WavFiles/CheckScribble2.CheckScribble2" 1.0 1.0 0.0 null null))

(event `self.Box.OnComponentEndOverlap`
  (params (OverlappedComponent :type "PrimitiveComponent Object Reference") (OtherActor :type "Actor Object Reference") (OtherComp :type "PrimitiveComponent Object Reference") (OtherBodyIndex :type Integer))
  (bind _outactors (`GameplayStatics.GetAllActorsOfClass` "BP_AISpawner_C"))
  (for _array_element _outactors
    (`self.K2_DestroyActor` _array_element)))

(fn `UserConstructionScript`)