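; BP_DrawerTransform is a drawer that slides open and closed, with configurable drawer and inner meshes.
; The construction script assigns both meshes, while Open and Close events each play their own timeline and update IsOpen.
; Each timeline update lerps the drawer's current relative location toward a fixed Y offset or the origin, so the motion compounds rather than interpolating from a stored start.
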(event `Open`
  (bind (_direction _newtrack_0) (`Timeline|Timeline_0` :!via `PlayFromStart`)
    (:`Update`
      (set `self.isOpen` true)
      (`SceneComponent.K2_SetRelativeLocation` (`self.Drawer Mesh`) (`KismetMathLibrary.VLerp` (`SceneComponent.RelativeLocation` (`self.Drawer Mesh`)) (0.0 26.0 0.0) _newtrack_0) false false))))

(event `Close`
  (bind (_direction _newtrack_0) (`Timeline|Timeline_1` :!via `PlayFromStart`)
    (:`Update`
      (set `self.isOpen` false)
      (`SceneComponent.K2_SetRelativeLocation` (`self.Drawer Mesh`) (`KismetMathLibrary.VLerp` (`SceneComponent.RelativeLocation` (`self.Drawer Mesh`)) (0.0 0.0 0.0) _newtrack_0) false false))))

(fn `UserConstructionScript`
  (`|ExecutionSequence`
    (:`then_0`
      (`StaticMeshComponent.SetStaticMesh` (`self.Drawer Mesh`) (`self.Drawer`)))
    (:`then_1`
      (`StaticMeshComponent.SetStaticMesh` (`self.InnerComponent`) (`self.InComponent`)))))