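; BP_LockerHide is a locker that the L1_Character can hide in and leave with the Action input.
; Overlapping its box enables input and opens a gate; leaving disables both.
; Action toggles the character's visibility and collision, blends the camera between locker and character, and plays a timeline-driven door rotation.
; Input and gate re-enable shortly after each toggle, independent of overlap.
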(event `InputAction|Action`
  (params (Key :type "Key Structure"))
  (:`Pressed`
    (`/Engine/EditorBlueprintResources/StandardMacros.Gate` true :!label _label
      (:`Exit`
        (`|ExecutionSequence`
          (:`then_0`
            (`self.ToggleHide`)
            (`KismetSystemLibrary.Delay` 0.2)
            (`self.EnableInput` (`GameplayStatics.GetPlayerController` 0) :!label _label_2)
            (goto _label :!via `Open`))
          (:`then_1`
            (bind (_direction _doortrack) (`Timeline|OpenCloseDoorT` :!via `PlayFromStart`)
              (:`Update`
                (`SceneComponent.K2_SetRelativeRotation` (`self.Locker_Door`) (`KismetMathLibrary.MakeRotator` 0.0 0.0 (`KismetMathLibrary.Lerp` (`self.ClosedAngle`) (`self.OpenedAngle`) _doortrack)) false false)))))))))

(event `self.Box.OnComponentBeginOverlap`
  (params (OverlappedComponent :type "PrimitiveComponent Object Reference") (OtherActor :type "Actor Object Reference") (OtherComp :type "PrimitiveComponent Object Reference") (OtherBodyIndex :type Integer) (bFromSweep :type Boolean) (SweepResult :type "HitResult Structure (by ref)"))
  (bind _asl1_character (cast `/Game/AnthonyStuff/Content/GameBP/Level1/L1_Character` OtherActor))
  (set `self.CharRef` _asl1_character)
  (goto _label_2))

(event `self.Box.OnComponentEndOverlap`
  (params (OverlappedComponent :type "PrimitiveComponent Object Reference") (OtherActor :type "Actor Object Reference") (OtherComp :type "PrimitiveComponent Object Reference") (OtherBodyIndex :type Integer))
  (cast `/Game/AnthonyStuff/Content/GameBP/Level1/L1_Character` OtherActor)
  (`self.DisableInput` (`GameplayStatics.GetPlayerController` 0))
  (goto _label :!via `Close`))

(fn `ToggleHide`
  (bind _returnvalue (`GameplayStatics.GetPlayerController` 0))
  (bind _charref (`self.CharRef`))
  (if (`self.isHiding?`)
    (set `self.isHiding?` false)
    (`self.SetActorHiddenInGame` _charref false)
    (`self.SetActorEnableCollision` _charref true)
    (`PlayerController.SetViewTargetWithBlend` _returnvalue _charref 0.8 "VTBlend_Linear" 0.0 false)
    (else
      (set `self.isHiding?` true)
      (`self.SetActorHiddenInGame` _charref true)
      (`self.SetActorEnableCollision` _charref false)
      (`PlayerController.SetViewTargetWithBlend` _returnvalue self 0.8 "VTBlend_Linear" 0.0 false))))

(fn `UserConstructionScript`)