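; Interactable hiding spot that moves the player between its hiding and exit positions and toggles their IsHiding state.
; Interact blocks time travel and starts a looping per-frame timer that slides the player at constant speed, disabling collision and movement on entry.
; On arrival it fires a finished-moving dispatcher, restoring collision, walking and time travel on exit.
; The AIC_Classic enemy controller is notified when hiding starts and when the player leaves.
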(event `self.ReceiveBeginPlay`
  (bind _asl1_character (cast `/Game/AnthonyStuff/Content/GameBP/Level1/L1_Character` (`GameplayStatics.GetPlayerCharacter` 0)))
  (set `self.PlayerRef` _asl1_character))

(event `/Game/AnthonyStuff/Content/BluePrints/Interface/BPI_Interaction.Interact`
  (bind _playerref (`self.PlayerRef`))
  (bind _playerref_2 (`self.PlayerRef`))
  (set `/Game/AnthonyStuff/Content/GameBP/Level1/L1_Character.canTimeTravel?` false _playerref)
  (if (`/Game/AnthonyStuff/Content/GameBP/Level1/L1_Character.isHiding` _playerref)
    (bind _returnvalue (`KismetSystemLibrary.K2_SetTimerDelegate` (delegate `MoveCharacter`) (`GameplayStatics.GetWorldDeltaSeconds`) true))
    (else
      (bind _asaic_classic (castclass `/Game/AnthonyStuff/Content/AI/Classic/AIC_Classic` "/Game/AnthonyStuff/Content/AI/Classic/AIC_Classic.AIC_Classic_C"))
      (bind _returnvalue_2 (`GameplayStatics.GetActorOfClass` _asaic_classic))
      (message `/Game/AnthonyStuff/Content/BluePrints/Interface/BPI_PlayerHiding.DidEnemySee` _returnvalue_2 self)
      (`self.SetActorEnableCollision` _playerref_2 false)
      (`CharacterMovementComponent.DisableMovement` (`Character.CharacterMovement` _playerref_2))
      (bind _returnvalue_3 (`KismetSystemLibrary.K2_SetTimerDelegate` (delegate `MoveCharacter`) (`GameplayStatics.GetWorldDeltaSeconds`) true)))))

(event `MoveCharacter`
  (bind _playerref (`self.PlayerRef`))
  (`self.K2_SetActorTransform` _playerref (`KismetMathLibrary.MakeTransform` (`KismetMathLibrary.VInterpTo_Constant` (`self.K2_GetActorLocation` _playerref) (`SceneComponent.K2_GetComponentLocation` (select `bool` (`/Game/AnthonyStuff/Content/GameBP/Level1/L1_Character.isHiding` (`self.PlayerRef`)) :`false` (`self.HidingPosition`) :`true` (`self.ExitPosition`))) (`GameplayStatics.GetWorldDeltaSeconds`) 1000.0)) false false)
  (if (== (`self.K2_GetActorLocation` (`self.PlayerRef`)) (`SceneComponent.K2_GetComponentLocation` (select `bool` (`/Game/AnthonyStuff/Content/GameBP/Level1/L1_Character.isHiding` (`self.PlayerRef`)) :`false` (`self.HidingPosition`) :`true` (`self.ExitPosition`) :!type "SceneComponent Object Reference")) :`ErrorTolerance` 0.01)
    (`KismetSystemLibrary.K2_ClearAndInvalidateTimerHandle` (stale `/Game/AnthonyStuff/Content/BluePrints/Interface/BPI_Interaction.Interact` _returnvalue_3))
    (`KismetSystemLibrary.K2_ClearAndInvalidateTimerHandle` (stale `/Game/AnthonyStuff/Content/BluePrints/Interface/BPI_Interaction.Interact` _returnvalue))
    (`self.FinishedMoving`)))

(event `FinishedMoving`
  (bind _playerref (`self.PlayerRef`))
  (bind _playerref_2 (`self.PlayerRef`))
  (`self.FinishedMovingED`)
  (if (`/Game/AnthonyStuff/Content/GameBP/Level1/L1_Character.isHiding` _playerref_2)
    (set `/Game/AnthonyStuff/Content/GameBP/Level1/L1_Character.isHiding` false _playerref_2)
    (bind _asaic_classic (castclass `/Game/AnthonyStuff/Content/AI/Classic/AIC_Classic` "/Game/AnthonyStuff/Content/AI/Classic/AIC_Classic.AIC_Classic_C"))
    (bind _returnvalue (`GameplayStatics.GetActorOfClass` _asaic_classic))
    (message `/Game/AnthonyStuff/Content/BluePrints/Interface/BPI_PlayerHiding.LeftHidingSpot` _returnvalue)
    (`self.SetActorEnableCollision` _playerref true)
    (`CharacterMovementComponent.SetMovementMode` (`Character.CharacterMovement` _playerref) "MOVE_Walking" 0)
    (set `/Game/AnthonyStuff/Content/GameBP/Level1/L1_Character.canTimeTravel?` true _playerref)
    (else
      (set `/Game/AnthonyStuff/Content/GameBP/Level1/L1_Character.isHiding` true _playerref_2))))

(event `EnemyFound`)

(fn `UserConstructionScript`)