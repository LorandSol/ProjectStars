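; Locker hiding spot, a child of a hide actor Blueprint, that animates its door with timeline-driven yaw rotation.
; Interact locks further interaction and swings the door open, then hands off to the parent's Interact.
; The inherited finished-moving dispatcher triggers the door to close, which re-enables interaction.
; EnemyFound disables interaction and door collision and opens the door through a separate AI timeline.
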(event `self.ReceiveBeginPlay`
  (`parent.ReceiveBeginPlay`)
  (add `self.FinishedMovingED` (delegate `FinishedMovingED_Event`)))

(event `FinishedMovingED_Event`
  (`KismetSystemLibrary.Delay` 0.1)
  (`self.CloseDoor`))

(event `/Game/AnthonyStuff/Content/BluePrints/Interface/BPI_Interaction.Interact`
  (if (`self.canInteract`)
    (set `self.canInteract` false)
    (bind (_direction _alpha) (`Timeline|OpenLockerDoor` :!via `PlayFromStart`)
      (:`Update`
        (`SceneComponent.K2_SetRelativeRotation` (`self.LockerDoor`) (`KismetMathLibrary.MakeRotator` 0.0 0.0 (`KismetMathLibrary.Lerp` 0.0 90.0 _alpha)) false false))
      (:`Finished`
        (`KismetSystemLibrary.Delay` 0.1)
        (`parent.Interact`)))))

(event `CloseDoor`
  (bind (_direction _alpha) (`Timeline|CloseLockerDoor` :!via `PlayFromStart`)
    (:`Update`
      (`SceneComponent.K2_SetRelativeRotation` (`self.LockerDoor`) (`KismetMathLibrary.MakeRotator` 0.0 0.0 (`KismetMathLibrary.Lerp` 90.0 0.0 _alpha)) false false))
    (:`Finished`
      (set `self.canInteract` true))))

(event `self.EnemyFound`
  (set `self.canInteract` false)
  (`PrimitiveComponent.SetCollisionEnabled` (`self.LockerDoor`) "NoCollision")
  (bind (_direction _alpha) (`Timeline|AIOpenDoor` :!via `PlayFromStart`)
    (:`Update`
      (`SceneComponent.K2_SetRelativeRotation` (`self.LockerDoor`) (`KismetMathLibrary.MakeRotator` 0.0 0.0 (`KismetMathLibrary.Lerp` 0.0 90.0 _alpha)) false false))
    (:`Finished`
      (`KismetSystemLibrary.Delay` 0.1))))

(fn `UserConstructionScript`
  (`parent.UserConstructionScript`))