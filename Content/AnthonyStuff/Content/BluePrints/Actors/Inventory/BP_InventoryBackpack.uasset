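; BP_InventoryBackpack is a world pickup that expands the player's inventory by adding slots when the Action input is pressed, then destroys itself.
; A sphere overlap with L1_Character starts per-tick checks and shows a prompt widget that floats above the mesh.
; Each tick a visibility trace to the player camera hides the prompt when blocked; otherwise it faces the camera, and pickup distance toggles prompt state and input.
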(event `self.Sphere.OnComponentBeginOverlap`
  (params (OverlappedComponent :type "PrimitiveComponent Object Reference") (OtherActor :type "Actor Object Reference") (OtherComp :type "PrimitiveComponent Object Reference") (OtherBodyIndex :type Integer) (bFromSweep :type Boolean) (SweepResult :type "HitResult Structure (by ref)"))
  (bind _asl1_character (cast `/Game/AnthonyStuff/Content/GameBP/Level1/L1_Character` OtherActor))
  (set `self.PlayerRef` _asl1_character)
  (`SceneComponent.SetVisibility` (`self.PickUpWidget`) true false)
  (set `self.UpdateActor` true))

(event `self.Sphere.OnComponentEndOverlap`
  (params (OverlappedComponent :type "PrimitiveComponent Object Reference") (OtherActor :type "Actor Object Reference") (OtherComp :type "PrimitiveComponent Object Reference") (OtherBodyIndex :type Integer))
  (cast `/Game/AnthonyStuff/Content/GameBP/Level1/L1_Character` OtherActor)
  (`SceneComponent.SetVisibility` (`self.PickUpWidget`) false false)
  (set `self.UpdateActor` false)
  (`self.DisableInput` (`GameplayStatics.GetPlayerController` 0)))

(event `self.ReceiveTick`
  (params (DeltaSeconds :type "Float (single-precision)"))
  (bind _returnvalue (`GameplayStatics.GetPlayerController` 0))
  (bind _pickupwidget (`self.PickUpWidget`))
  (bind (_returnvalue_x _returnvalue_y _returnvalue_z) (`KismetMathLibrary.BreakVector` (`SceneComponent.K2_GetComponentLocation` (`self.StaticMesh`))))
  (`SceneComponent.K2_SetWorldLocation` (`self.PickUpWidget`) (`KismetMathLibrary.MakeVector` _returnvalue_x _returnvalue_y (+ _returnvalue_z (`self.WidgetDistanceAboveMesh`))) false false)
  (if (`self.UpdateActor`)
    (bind (_outhit _returnvalue_2) (`KismetSystemLibrary.LineTraceSingle` (`self.K2_GetActorLocation`) (`SceneComponent.K2_GetComponentLocation` (`/Game/AnthonyStuff/Content/GameBP/Level1/L1_Character.Camera` (`self.PlayerRef`))) "TraceTypeQuery1"))
    (if (not _returnvalue_2)
      (`SceneComponent.SetVisibility` _pickupwidget true false)
      (`SceneComponent.K2_SetWorldRotation` (`self.PickUpWidget`) (`KismetMathLibrary.FindLookAtRotation` (`SceneComponent.K2_GetComponentLocation` (`self.PickUpWidget`)) (`SceneComponent.K2_GetComponentLocation` (`/Game/AnthonyStuff/Content/GameBP/Level1/L1_Character.Camera` (`self.PlayerRef`)))) false false)
      (bind (_bblockinghit _binitialoverlap _time _distance _location _impactpoint _normal _impactnormal _physmat _hitactor _hitcomponent _hitbonename _bonename _hititem _elementindex _faceindex _tracestart _traceend) (`GameplayStatics.BreakHitResult` _outhit))
      (bind _returnvalue_3 (<= (`KismetMathLibrary.VSize` (- _tracestart _traceend)) (`self.PickUpDistance`)))
      (`/Game/AnthonyStuff/Content/UMG/Inventory/W_PickUpPrompt.TogglePrompt` (cast `/Game/AnthonyStuff/Content/UMG/Inventory/W_PickUpPrompt` (`WidgetComponent.GetUserWidgetObject` (`self.PickUpWidget`)) :!pure true) _returnvalue_3)
      (if _returnvalue_3
        (`self.EnableInput` _returnvalue)
        (else
          (`self.DisableInput` _returnvalue)))
      (else
        (`SceneComponent.SetVisibility` _pickupwidget false false)
        (`self.DisableInput` (`GameplayStatics.GetPlayerController` 0))))))

(event `InputAction|Action`
  (params (Key :type "Key Structure"))
  (:`Pressed`
    (`/Game/AnthonyStuff/Content/BluePrints/BluePrintComponents/BPC_Inventory.AddMoreSlots` (`/Game/AnthonyStuff/Content/GameBP/Level1/L1_Character.BPC_Inventory` (`self.PlayerRef`)) (`self.AmountOfSlots`))
    (`self.K2_DestroyActor`)))

(fn `UserConstructionScript`)