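; BP_TestNote is an interactable note that toggles between lying in the world and being read on screen.
; Interact flips HoldingNote: picking up hides the note's actor, shows a TestNote_widget, disables L1_Character movement and disables HG_PlayerController input.
; The next Interact removes the widget, unhides the note and restores walking and controller input.
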(event `/Game/Blueprints/Interface/BPI_Interaction.Interact`
  (if (not (`self.HoldingNote?`))
    (set `self.HoldingNote?` true)
    (`self.SetActorHiddenInGame` (`ActorComponent.GetOwner` (`self.TestNote`)) true)
    (bind _returnvalue (`|CreateWidget` "/Game/LaylaStuff/Blueprints/TestNote_widget.TestNote_widget_C"))
    (bind _output_get (set `self.NoteWidgetRef` _returnvalue))
    (`UserWidget.AddToViewport` _output_get 0)
    (bind _asl1_character (cast `/Game/Blueprints/PlayerCharacter/Level1/L1_Character` (`GameplayStatics.GetPlayerCharacter` 0)))
    (`CharacterMovementComponent.DisableMovement` (`Character.CharacterMovement` _asl1_character))
    (bind _ashg_player_controller (cast `/Game/Blueprints/PlayerCharacter/HG_PlayerController` (`GameplayStatics.GetPlayerController` 0)))
    (`self.DisableInput` _ashg_player_controller _ashg_player_controller)
    (else
      (set `self.HoldingNote?` false)
      (`Widget.RemoveFromParent` (`self.NoteWidgetRef`))
      (`self.SetActorHiddenInGame` (`ActorComponent.GetOwner` (`self.TestNote`)) false)
      (bind _asl1_character_2 (cast `/Game/Blueprints/PlayerCharacter/Level1/L1_Character` (`GameplayStatics.GetPlayerCharacter` 0)))
      (`CharacterMovementComponent.SetMovementMode` (`Character.CharacterMovement` _asl1_character_2) "MOVE_Walking" 0)
      (bind _ashg_player_controller_2 (cast `/Game/Blueprints/PlayerCharacter/HG_PlayerController` (`GameplayStatics.GetPlayerController` 0)))
      (`self.EnableInput` _ashg_player_controller_2 _ashg_player_controller_2))))

(fn `UserConstructionScript`)