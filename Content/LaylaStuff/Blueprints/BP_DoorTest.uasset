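; BP_DoorTest is a locked exit door that ends the game with a survival screen.
; Overlapping DoorCollision as an L1_Character with HasKey plays the DoorOpen timeline to rotate the door's yaw; without the key, a hint prints.
; The win sequence hangs off the timeline's Update: after a short delay it pauses the game, clears widgets, shows YouSurvivedWidget and enables the mouse cursor.
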(event `self.DoorCollision.OnComponentBeginOverlap`
  (params (OverlappedComponent :type "PrimitiveComponent Object Reference") (OtherActor :type "Actor Object Reference") (OtherComp :type "PrimitiveComponent Object Reference") (OtherBodyIndex :type Integer) (bFromSweep :type Boolean) (SweepResult :type "HitResult Structure (by ref)"))
  (bind _returnvalue (`GameplayStatics.GetPlayerController` 0))
  (bind _asl1_character (cast `/Game/AnthonyStuff/Content/GameBP/Level1/L1_Character` OtherActor))
  (if (`/Game/AnthonyStuff/Content/GameBP/Level1/L1_Character.HasKey` _asl1_character)
    (bind (_direction _doorrotation) (`Timeline|DoorOpen`)
      (:`Update`
        (`SceneComponent.K2_SetRelativeRotation` (`self.Door`) (`KismetMathLibrary.MakeRotator` 0.0 0.0 _doorrotation) false false)
        (`KismetSystemLibrary.Delay` 1.0)
        (`GameplayStatics.SetGamePaused` true)
        (`WidgetLayoutLibrary.RemoveAllWidgets`)
        (bind _returnvalue_2 (`|CreateWidget` "/Game/Widgets/YouSurvivedWidget.YouSurvivedWidget_C" _returnvalue))
        (`UserWidget.AddToViewport` _returnvalue_2 0)
        (set `PlayerController.bShowMouseCursor` true _returnvalue)))
    (else
      (`KismetSystemLibrary.PrintString` "Find Key to unlock door"))))

(fn `UserConstructionScript`)