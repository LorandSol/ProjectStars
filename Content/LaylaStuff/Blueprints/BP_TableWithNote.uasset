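; BP_TableWithNote is a table actor that toggles a readable note on screen with the Action input.
; On press, it stores the Table component and, if that object is named "Note", hides the owning actor and shows a new TestNote_widget.
; The next press removes the widget and unhides the actor, with a HoldingNote flag tracking the state.
; The input handler has no proximity or trace check.
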(event `InputAction|Action`
  (params (Key :type "Key Structure"))
  (:`Pressed`
    (if (not (`self.HoldingNote?`))
      (bind _output_get (set `self.StaticMeshRef` (`self.Table`)))
      (if (`KismetStringLibrary.EqualEqual_StrStr` (`KismetSystemLibrary.GetObjectName` _output_get) "Note")
        (set `self.HoldingNote?` true)
        (`self.SetActorHiddenInGame` (`ActorComponent.GetOwner` _output_get) true)
        (bind _returnvalue (`|CreateWidget` "/Game/LaylaStuff/Blueprints/TestNote_widget.TestNote_widget_C"))
        (bind _output_get_2 (set `self.NoteRef` _returnvalue))
        (`UserWidget.AddToViewport` _output_get_2 0))
      (else
        (set `self.HoldingNote?` false)
        (`Widget.RemoveFromParent` (`self.NoteRef`))
        (`self.SetActorHiddenInGame` (`ActorComponent.GetOwner` (`self.StaticMeshRef`)) false)))))

(fn `UserConstructionScript`)