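; Vintage bedroom prop Blueprint for a drawer part that rotates open and closed through Open and Close events.
; Each event plays its own timeline, which updates IsOpen and lerps DrawerMesh's relative rotation toward a quarter turn or back to zero.
; The lerp starts from the current rotation on every update, so the motion compounds rather than following the curve directly.
; The construction script assigns the mesh from the Drawer variable.
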(event `Open`
  (bind (_direction _newtrack_0) (`Timeline|Timeline_0` :!via `PlayFromStart`)
    (:`Update`
      (set `self.isOpen` true)
      (`SceneComponent.K2_SetRelativeRotation` (`self.Drawer Mesh`) (`KismetMathLibrary.RLerp` (`SceneComponent.RelativeRotation` (`self.Drawer Mesh`)) (struct :`Yaw` 90.0) _newtrack_0) false false))))

(event `Close`
  (bind (_direction _newtrack_0) (`Timeline|Timeline_1` :!via `PlayFromStart`)
    (:`Update`
      (set `self.isOpen` false)
      (`SceneComponent.K2_SetRelativeRotation` (`self.Drawer Mesh`) (`KismetMathLibrary.RLerp` (`SceneComponent.RelativeRotation` (`self.Drawer Mesh`)) (struct) _newtrack_0) false false))))

(fn `UserConstructionScript`
  (`StaticMeshComponent.SetStaticMesh` (`self.Drawer Mesh`) (`self.Drawer`)))